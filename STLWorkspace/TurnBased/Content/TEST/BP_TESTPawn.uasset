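; Test pawn whose cube reacts to mouse hover and clicks on its box.
; Hover swaps the cube to a new material, and cursor exit restores the original cached at BeginPlay unless the pawn is clicked.
; A click applies that material, stores and prints the actor's location, and sets a flag.
; Tick sees the flag, disables the player controller's click and mouse-over events, then re-enables them and clears it after a delay.
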(event `self.ReceiveBeginPlay`
  ;[1 1 1] 원래 마테리얼 저장
  (set `self.OriginMaterial` (`PrimitiveComponent.GetMaterial` (`self.Cube`) 0)))

(event `self.ReceiveTick`
  (params (DeltaSeconds :type "Float (single-precision)"))
  (bind _returnvalue (`GameplayStatics.GetPlayerController` 0))
  (bind _returnvalue_2 (`GameplayStatics.GetPlayerController` 0))
  (if (`self.IsClicked`)
    (set `PlayerController.bEnableMouseOverEvents` false _returnvalue)
    (set `PlayerController.bEnableClickEvents` false _returnvalue)
    (`KismetSystemLibrary.Delay` 3.0) ; 딜레이 후, 원상태로 돌아옴
    (set `PlayerController.bEnableMouseOverEvents` true _returnvalue_2)
    (set `PlayerController.bEnableClickEvents` true _returnvalue_2)
    (set `self.IsClicked` false)))

(event `self.Box.OnClicked`
  (params (TouchedComponent :type "PrimitiveComponent Object Reference") (ButtonPressed :type "Key Structure"))
  ;[1 1 1] 클릭
  (`PrimitiveComponent.SetMaterial` (`self.Cube`) 0 "/Game/TEST/NewMaterial.NewMaterial")
  (set `self.IsClicked` true)
  ;[1 1 1] 클릭된 오브제 위치 저장
  (bind _output_get (set `self.TargetLoc` (`self.K2_GetActorLocation`)))
  (`KismetSystemLibrary.PrintString` (`KismetStringLibrary.Conv_VectorToString` _output_get)))

(event `self.Box.OnBeginCursorOver`
  (params (TouchedComponent :type "PrimitiveComponent Object Reference"))
  ;[1 1 1] 커서 오버랩
  (`PrimitiveComponent.SetMaterial` (`self.Cube`) 0 "/Game/TEST/NewMaterial.NewMaterial"))

(event `self.Box.OnEndCursorOver`
  (params (TouchedComponent :type "PrimitiveComponent Object Reference"))
  ;[1 1 1] 커서 오버랩
  (if (not (`self.IsClicked`))
    (`PrimitiveComponent.SetMaterial` (`self.Cube`) 0 (`self.OriginMaterial`))))

(fn `UserConstructionScript`)