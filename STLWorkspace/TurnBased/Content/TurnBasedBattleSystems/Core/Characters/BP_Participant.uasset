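; Battle participant character for a turn-based combat system, controlled by the player or random AI depending on team.
; It registers with the game mode, which it notifies when actions end.
; Turns open an action menu or pick random targets for a move-and-punch attack or explosion spell, executed immediately or stored for preselect modes.
; It also handles damage, death, widget-component health and damage displays, team colours and custom-depth target highlighting.
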(event `self.ReceiveBeginPlay`
  ;[1 1 1] Begin play
  ;;[1 1 1] Add to participant list when spawned
  (bind _gamemode (`self.GetGameMode`))
  (bind _successful (`/Game/TurnBasedBattleSystems/Core/GameModes/BP_TurnBasedGameMode.AddParticipant` _gamemode self))
  (if _successful
    ;[1 1 1] Set up health bar
    ;;[1 1 1] Create the health widget
    (bind _returnvalue (`|CreateWidget` "/Game/TurnBasedBattleSystems/UI/WBP_HealthBar.WBP_HealthBar_C" null self))
    (set `self.HealthBarWidgetReference` _returnvalue)
    ;;[1 1 1] Create the 3D widget component
    (bind _returnvalue_2 (`AddComponent|NODE_AddWidgetComponent-1` :`bManualAttachment` true :`RelativeTransform` (`KismetMathLibrary.MakeTransform` (0.0 0.0 120.0) (struct :`Pitch` 20.0 :`Yaw` 180.0) (1.0 1.0 1.0))))
    (bind _output_get (set `self.HealthBarWidgetComponent` _returnvalue_2))
    ;;[1 1 1] Set the 3D widget to the health widget
    (`WidgetComponent.SetWidget` _output_get (`self.HealthBarWidgetReference`))
    ;;[1 1 1] Turn off absolute rotation
    (set `SceneComponent.bAbsoluteRotation` true (`self.HealthBarWidgetComponent`))
    ;;[1 1 1] Attach to the capsule component
    (`SceneComponent.K2_AttachToComponent` (`self.HealthBarWidgetComponent`) (`self.CapsuleComponent`) "None" "KeepRelative" "KeepRelative" "KeepRelative" true)))

(event `self.ReceiveTick`
  (params (DeltaSeconds :type "Float (single-precision)"))
  ;[1 1 1] Tick
  (`self.SmoothRotation` DeltaSeconds))

(event `self.ReceiveAnyDamage`
  (params (Damage :type "Float (single-precision)") (DamageType :type "DamageType Object Reference") (InstigatedBy :type "Controller Object Reference") (DamageCauser :type "Actor Object Reference"))
  ;[1 1 1] Take damage event
  (bind _output_get (set `self.DamageTaken` Damage))
  ;;[1 1 1] Create widget
  (`self.CreateDamageWidget` _output_get)
  ;;[1 1 1] Set health
  (bind _output_get_2 (set `self.Health` (- (`self.Health`) (`self.DamageTaken`))))
  (if (<= _output_get_2 0.0)
    ;;[1 1 1] If health under or equal to zero, die
    (`self.Die`)
    (else
      ;;[1 1 1] If health above zero, set the anim blueprint flag for taking damage animation
      (set `self.TakingDamage` true)
      ;;[1 1 1] Reset flag after animation complete
      (`KismetSystemLibrary.Delay` 0.967)
      (set `self.TakingDamage` false))))

(event `NotFinishedRotating`
  (bind (_initialtransform_location _initialtransform_rotation) (`KismetMathLibrary.BreakTransform` (`self.InitialTransform`)))
  ;[1 1 1] Move to attack
  ;;[1 1 1] Wait until we have finished rotating
  (`KismetSystemLibrary.Delay` 0.01 :!label _label)
  (if (`self.SmoothRotate`)
    (`self.NotFinishedRotating`)
    (else
      ;;[1 1 1] Play punching animation and reset after a delay
      (set `self.Punching` true)
      (`self.DealDamage` (`self.TargetParticipant`))
      (`KismetSystemLibrary.Delay` 0.778)
      (set `self.Punching` false)
      ;;[1 1 1] Move and rotate back to original position
      (`|AIMoveTo` self _initialtransform_location
        (:`OnSuccess`
          (set `self.DesiredRotation` _initialtransform_rotation)
          (set `self.SmoothRotate` true)
          ;;[1 1 1] End our turn after a delay
          (`KismetSystemLibrary.Delay` 0.5)
          (`self.EndAction`))))))

(event `MoveToAttack`
  (params (TargetParticipant :type "/Game/TurnBasedBattleSystems/Core/Characters/BP_Participant Object Reference"))
  (bind (_returnvalue_roll _returnvalue_pitch _returnvalue_yaw) (`KismetMathLibrary.BreakRotator` (`self.K2_GetActorRotation` (`self.TargetParticipant`))))
  ;[1 1 1] Move to attack
  ;;[1 1 1] Store the target participant
  (set `self.TargetParticipant` TargetParticipant)
  ;;[1 1 1] Set our initial transform
  (set `self.InitialTransform` (`self.GetTransform`))
  ;;[1 1 1] Set our movement target to 100 units in front of target participant
  (`|AIMoveTo` self (+ (`self.K2_GetActorLocation` (`self.TargetParticipant`)) (* (`self.GetActorForwardVector` (`self.TargetParticipant`)) 100.0))
    (:`OnSuccess`
      ;;[1 1 1] Once arravied, set our desired rotation to face the target participant and set the smooth rotate flag
      (set `self.DesiredRotation` (`KismetMathLibrary.MakeRotator` 0.0 0.0 (+ _returnvalue_yaw 180.0)))
      (set `self.SmoothRotate` true)
      (goto _label))
    (:`OnFail`
      ;;[1 1 1] Print an error string if failed
      (`KismetSystemLibrary.PrintString` "Movement failed, ensure you have nav mesh for level geometry"))))

(event `CastSpellAtTarget`
  (params (TargetParticipant :type "/Game/TurnBasedBattleSystems/Core/Characters/BP_Participant Object Reference"))
  ;[1 1 1] Spell
  ;;[1 1 1] After a delay, create an explosion at target location
  (`KismetSystemLibrary.Delay` 0.2)
  (bind _output_get (set `self.TargetParticipant` TargetParticipant))
  (`GameplayStatics.SpawnEmitterAtLocation` "/Game/TurnBasedBattleSystems/Effects/P_Explosion_Fireball.P_Explosion_Fireball" (`self.K2_GetActorLocation` _output_get))
  ;;[1 1 1] Play a sound and make the participant jump
  (`GameplayStatics.PlaySound2D` "/Game/TurnBasedBattleSystems/Audio/Cue/S_Spell_Cue.S_Spell_Cue")
  (`self.Jump`)
  ;;[1 1 1] After a delay, deal damage
  (`KismetSystemLibrary.Delay` 0.2)
  (`self.DealDamage` (`self.TargetParticipant`))
  (`KismetSystemLibrary.Delay` 1.5)
  ;;[1 1 1] End the participant's action
  (`self.EndAction`))

(event `FlashTurnMarker`
  ;[1 1 1] Flash Turn Marker
  ;;[1 1 1] If we are controlled by the player
  (bind _iscontrolledteam (`self.CheckControlledTeam`))
  (if _iscontrolledteam
    ;;[1 1 1] Play a timeline to set turn marker opacity over time
    (bind (_direction _opacity) (`Timeline|TurnMarkerFlash` :!via `PlayFromStart`)
      (:`Update`
        (`MaterialInstanceDynamic.SetScalarParameterValue` (`self.TurnMarkerDI`) "Opacity" _opacity)))))

(fn `ActionSuccessful`
  (locals (ChargeUpGameMode :type "/Game/TurnBasedBattleSystems/Core/GameModes/ChargeUp/BP_ChargeUpGameMode Object Reference"))
  ;[1 1 1] Remove widget
  (`Widget.RemoveFromParent` (`self.ActionSelectWidget`))
  ;[1 0.9267 0] Pause charge on action (charge up specific)
  ;;[1 1 1] Store the game mode if is of type Charge Up Game Mode
  (bind _gamemode (`self.GetGameMode`))
  (bind _asbp_charge_up_game_mode (cast `/Game/TurnBasedBattleSystems/Core/GameModes/ChargeUp/BP_ChargeUpGameMode` _gamemode))
  (set `local.ChargeUpGameMode` _asbp_charge_up_game_mode)
  ;;[1 1 1] Pause if Pause On Action is current mode
  (if (`|EnumEquality` (`/Game/TurnBasedBattleSystems/Core/GameModes/ChargeUp/BP_ChargeUpGameMode.Mode` (`local.ChargeUpGameMode`)) "NewEnumerator1")
    (set `/Game/TurnBasedBattleSystems/Core/GameModes/ChargeUp/BP_ChargeUpGameMode.Pause` true (`local.ChargeUpGameMode`))))

(fn `AIControlledAction`
  (locals (PotentialTargets :type "Array of /Game/TurnBasedBattleSystems/Core/Characters/BP_Participant Object Reference") (CurrentParticipant :type "/Game/TurnBasedBattleSystems/Core/Characters/BP_Participant Object Reference") (GameMode :type "/Game/TurnBasedBattleSystems/Core/GameModes/BP_TurnBasedGameMode Object Reference"))
  (bind _potentialtargets (`local.PotentialTargets`))
  ;[1 1 1] Create a list of participants on teams other than the players team.
  (bind _gamemode (`self.GetGameMode`))
  (for _array_element (`/Game/TurnBasedBattleSystems/Core/GameModes/BP_TurnBasedGameMode.Participants` _gamemode)
    (bind _output_get (set `local.CurrentParticipant` _array_element))
    (if (not (not (!= (`/Game/TurnBasedBattleSystems/Core/Characters/BP_Participant.Team` _output_get) (`self.Team`))))
      (`KismetArrayLibrary.Array_AddUnique` (`local.PotentialTargets`) (`local.CurrentParticipant`))))
  ;[1 1 1] Pick a random participant from the list and attack them.
  (bind _output_get_2 (set `local.CurrentParticipant` (`KismetArrayLibrary.Array_Get` _potentialtargets (`KismetMathLibrary.RandomIntegerInRange` 0 (`KismetArrayLibrary.Array_LastIndex` _potentialtargets)))))
  (`/Engine/EditorBlueprintResources/StandardMacros.IsValid` _output_get_2
    (:`Is Valid`
      ;[1 1 1] Set preselect target or attack/spell
      ;;[1 1 1] Get the value of preselect from the game mode
      (bind _gamemode_2 (`self.GetGameMode`))
      (bind _output_get_3 (set `local.GameMode` _gamemode_2))
      (if (`/Game/TurnBasedBattleSystems/Core/GameModes/BP_TurnBasedGameMode.Preselect` _output_get_3)
        ;;[1 1 1] Preselct is true, set future action
        (set `self.PreselectTarget` (`local.CurrentParticipant`))
        (`/Game/TurnBasedBattleSystems/Core/GameModes/BP_TurnBasedGameMode.ParticipantEndAction` (`local.GameMode`) self)
        (set `self.ActionState` (select `bool` (`KismetMathLibrary.RandomBool`) :`false` "NewEnumerator1" :`true` "NewEnumerator2" :!type "/Game/TurnBasedBattleSystems/Core/Characters/Enumerations/ActionState Enum"))
        (else
          ;;[1 1 1] Preselect is false, do action immediately
          ;;;[1 1 1] Show enemy turn info widget
          (`self.CreateInfoTextWidget` "Enemy Turn!")
          (if (`KismetMathLibrary.RandomBool`)
            (`self.MoveToAttack` (`local.CurrentParticipant`))
            (else
              (`self.CastSpellAtTarget` (`local.CurrentParticipant`)))))))))

(fn `CheckControlledTeam`
  (returns (IsControlledTeam :type Boolean))
  ;[1 1 1] Try cast to Battle Controller
  (bind _asbp_battle_controller (cast `/Game/TurnBasedBattleSystems/Core/Characters/BP_BattleController` (`GameplayStatics.GetPlayerController` 0))
    (:`then`
      ;[1 1 1] Returns if this participants team is the game modes controlled team
      (return (== (`/Game/TurnBasedBattleSystems/Core/Characters/BP_BattleController.ControlledTeam` _asbp_battle_controller) (`self.Team`))))
    (:`CastFailed`
      ;[1 1 1] Show error message
      (`KismetSystemLibrary.PrintString` "Couldn't cast to turn based game mode!" false)
      (return false))))

(fn `CheckOurTurn`
  (returns (OurTurn :type Boolean))
  (bind _asbp_turn_based_game_mode (cast `/Game/TurnBasedBattleSystems/Core/GameModes/BP_TurnBasedGameMode` (`GameplayStatics.GetGameMode`))
    (:`then`
      ;[1 1 1] Check we are the current participant and return true if so
      (return (== (`/Game/TurnBasedBattleSystems/Core/GameModes/BP_TurnBasedGameMode.CurrentParticipant` _asbp_turn_based_game_mode) self)))
    (:`CastFailed`
      ;[1 1 1] Return false if we couldn't cast and show an error
      (`KismetSystemLibrary.PrintString` "Couldn't cast to turn based game mode!" false)
      (return false))))

(fn `CheckWon`
  (returns (Victory :type Boolean))
  (locals (NotAllDead :type Boolean) (CurrentParticipant :type "/Game/TurnBasedBattleSystems/Core/Characters/BP_Participant Object Reference"))
  (bind _currentparticipant (`local.CurrentParticipant`))
  ;[1 1 1] Loop all participants
  (bind _gamemode (`self.GetGameMode`))
  (for _array_element (`/Game/TurnBasedBattleSystems/Core/GameModes/BP_TurnBasedGameMode.Participants` _gamemode)
    (set `local.CurrentParticipant` _array_element)
    ;[1 1 1] If a participant on our team is not dead, set return value
    (if (and (not (`/Game/TurnBasedBattleSystems/Core/Characters/BP_Participant.Dead` _currentparticipant)) (!= (`/Game/TurnBasedBattleSystems/Core/Characters/BP_Participant.Team` _currentparticipant) (`self.Team`)))
      (set `local.NotAllDead` true)))
  ;[1 1 1] Return true if all team members dead
  (return (not (`local.NotAllDead`))))

(fn `CreateDamageWidget`
  (params (Damage :type "Float (double-precision)"))
  (locals (DamageWidgetReference :type "/Game/TurnBasedBattleSystems/UI/WBP_DamageWidget Object Reference") (DamageWidgetComponent :type "WidgetComponent Object Reference"))
  (bind _damagewidgetcomponent (`local.DamageWidgetComponent`))
  ;[1 1 1] Create widget and add component to render in 3D
  ;;[1 1 1] Create a damage widget
  (bind _returnvalue (`|CreateWidget` "/Game/TurnBasedBattleSystems/UI/WBP_DamageWidget.WBP_DamageWidget_C" null Damage))
  (set `local.DamageWidgetReference` _returnvalue)
  ;;[1 1 1] Create a 3D widget component
  (bind _returnvalue_2 (`AddComponent|NODE_AddWidgetComponent-2` :`bManualAttachment` true :`RelativeTransform` (`KismetMathLibrary.MakeTransform` (0.0 0.0 60.0) (struct :`Pitch` 20.0 :`Yaw` 180.0))))
  (bind _output_get (set `local.DamageWidgetComponent` _returnvalue_2))
  ;;[1 1 1] Set the 3D widget to the damage widget
  (`WidgetComponent.SetWidget` _output_get (`local.DamageWidgetReference`))
  ;;[1 1 1] Set the absolute rotation enabled and attach to the capsule compnent
  (set `SceneComponent.bAbsoluteRotation` true _damagewidgetcomponent)
  (`SceneComponent.K2_AttachToComponent` _damagewidgetcomponent (`self.CapsuleComponent`) "None" "KeepRelative" "KeepRelative" "KeepRelative" true))

(fn `CreateInfoTextWidget`
  (params (InfoString :type String))
  ;[1 1 1] Add a widget displaying simple information to the screen
  (bind _returnvalue (`|CreateWidget` "/Game/TurnBasedBattleSystems/UI/WBP_InfoText.WBP_InfoText_C" null InfoString))
  (`UserWidget.AddToViewport` _returnvalue 0))

(fn `DealDamage`
  (params (DamageTarget :type "/Game/TurnBasedBattleSystems/Core/Characters/BP_Participant Object Reference"))
  (bind _returnvalue (- (`self.Attack`) (`/Game/TurnBasedBattleSystems/Core/Characters/BP_Participant.Defence` DamageTarget)))
  ;[1 1 1] Very simple damage calculation example
  (`GameplayStatics.ApplyDamage` DamageTarget (`KismetMathLibrary.FClamp` _returnvalue 0.0 _returnvalue)))

(fn `Die`
  ;[1 1 1] Set dead
  (set `self.Dead` true)
  ;[1 1 1] Disable highlight
  (`self.Highlight` false)
  ;[1 1 1] Remove participant from list
  (bind _gamemode (`self.GetGameMode`))
  (`/Game/TurnBasedBattleSystems/Core/GameModes/BP_TurnBasedGameMode.RemoveParticipant` _gamemode self))

(fn `EndAction`
  ;[1 1 1] Reset menu and action state
  (set `self.MenuActionState` "NewEnumerator0")
  (set `self.ActionState` "NewEnumerator0")
  ;[1 1 1] Execute game mode end action code
  (bind _gamemode (`self.GetGameMode`))
  (`/Game/TurnBasedBattleSystems/Core/GameModes/BP_TurnBasedGameMode.ParticipantEndAction` _gamemode self))

(fn `ExecutePreselectedAction`
  (bind _preselecttarget (`self.PreselectTarget`))
  ;[1 1 1] Switch on action state
  (switch `/Game/TurnBasedBattleSystems/Core/Characters/Enumerations/ActionState` (`self.ActionState`)
    (:`NewEnumerator0`
      ;;[1 1 1] Default - End Action
      (`self.EndAction`))
    (:`NewEnumerator1`
      ;;[1 1 1] Attack
      (`self.MoveToAttack` _preselecttarget))
    (:`NewEnumerator2`
      ;;[1 1 1] Cast Spell
      (`self.CastSpellAtTarget` _preselecttarget))))

(fn `Highlight`
  (params (`Enable/Disable` :type Boolean) (Value :type "LinearColor Structure"))
  (locals (NewHighlightValue :type Boolean) (ColourValue :type "LinearColor Structure"))
  ;[1 1 1] Store the new highlight value and new colour
  (set `local.NewHighlightValue` `Enable/Disable`)
  (set `local.ColourValue` Value)
  ;[1 1 1] Flag render custom depth to show highlight, and set highlight color
  (bind _gamemode (`self.GetGameMode`))
  (`MaterialInstanceDynamic.SetVectorParameterValue` (`/Game/TurnBasedBattleSystems/Core/GameModes/BP_TurnBasedGameMode.HighlightMaterial` _gamemode) "Colour" (`local.ColourValue`))
  (`PrimitiveComponent.SetRenderCustomDepth` (`self.Mesh`) (`local.NewHighlightValue`)))

(fn `InitiateCombat`
  (locals (IsControlledTeam :type Boolean))
  ;[1 1 1] Set color based on team
  ;;[1 1 1] Store if we are controlled by the player
  (bind _iscontrolledteam (`self.CheckControlledTeam`))
  (set `local.IsControlledTeam` _iscontrolledteam)
  ;;[1 1 1] Create icon depending on team
  (bind _returnvalue (`|CreateWidget` "/Game/TurnBasedBattleSystems/UI/WBP_TurnOrderItem.WBP_TurnOrderItem_C" null (select `bool` (`local.IsControlledTeam`) :`false` "/Game/TurnBasedBattleSystems/UI/Textures/T_RedIcon.T_RedIcon" :`true` "/Game/TurnBasedBattleSystems/UI/Textures/T_GreenIcon.T_GreenIcon" :!type "Texture2D Object Reference") (`self.Name`)))
  (set `self.MyTurnOrderWidget` _returnvalue)
  ;;[1 1 1] Set colour depending on team
  (if (`local.IsControlledTeam`)
    (`self.SetColor` (struct :`G` 1.0 :`B` 0.190679 :`A` 1.0))
    (else
      (`self.SetColor` (struct :`R` 1.0 :`A` 1.0)))))

(fn `PlayerControlledAction`
  ;[1 1 1] Check the action select widget is valid
  (`self.ActionSelectWidget`
    (:`then`
      _)
    (:`else`
      ;[1 1 1] Create the menu widget
      (bind _returnvalue (`|CreateWidget` "/Game/TurnBasedBattleSystems/UI/WBP_ActionSelection.WBP_ActionSelection_C" null self))
      (set `self.ActionSelectWidget` _returnvalue)))
  ;[1 1 1] Add to screen
  (`UserWidget.AddToViewport` (`self.ActionSelectWidget`) 0)
  ;[1 1 1] If we aren't in a preselect game mode
  (bind _gamemode (`self.GetGameMode`))
  (if (not (`/Game/TurnBasedBattleSystems/Core/GameModes/BP_TurnBasedGameMode.Preselect` _gamemode))
    ;[1 1 1] Show player turn info widget
    (`self.CreateInfoTextWidget` "Player Turn!")))

(fn `PreselectedAction`
  (locals (CurrentParticipantList :type "Array of /Game/TurnBasedBattleSystems/Core/Characters/BP_Participant Object Reference"))
  ;[1 1 1] Safety net to prevent loops
  (bind _victory (`self.CheckWon`))
  (if (not _victory)
    ;[1 1 1] If dead end turn
    (if (not (`self.Dead`))
      ;[1 1 1] If our target isn't valid, pick a random new one
      ;;[1 1 1] Check our target is valid and not dead
      (if (and (not (`/Game/TurnBasedBattleSystems/Core/Characters/BP_Participant.Dead` (`self.PreselectTarget`))) (`KismetSystemLibrary.IsValid` (`self.PreselectTarget`)))
        ;;[1 1 1] True, so execute action
        (`self.ExecutePreselectedAction`)
        (else
          ;;[1 1 1] Get a list of participants
          (bind _gamemode (`self.GetGameMode`))
          (set `local.CurrentParticipantList` (`/Game/TurnBasedBattleSystems/Core/GameModes/BP_TurnBasedGameMode.Participants` _gamemode))
          ;;[1 1 1] While participant is dead, not valid, or on the same team as this participant
          (while (or (`/Game/TurnBasedBattleSystems/Core/Characters/BP_Participant.Dead` (`self.PreselectTarget`)) (not (`KismetSystemLibrary.IsValid` (`self.PreselectTarget`))) (== (`/Game/TurnBasedBattleSystems/Core/Characters/BP_Participant.Team` (`self.PreselectTarget`)) (`self.Team`)))
            ;;[1 1 1] Set a random participant as preselect target
            (set `self.PreselectTarget` (`self.GetRandomParticipant` (`local.CurrentParticipantList`))))
          ;;[1 1 1] Valid participant, execute action
          (`self.ExecutePreselectedAction`)))
      (else
        (`self.EndAction`)))))

(fn `RecieveInput`
  (params (Controller :type "/Game/TurnBasedBattleSystems/Core/Characters/BP_BattleController Object Reference"))
  (locals (ControllerReference :type "/Game/TurnBasedBattleSystems/Core/Characters/BP_BattleController Object Reference") (ParticipantUnderCursor :type "/Game/TurnBasedBattleSystems/Core/Characters/BP_Participant Object Reference") (GameMode :type "/Game/TurnBasedBattleSystems/Core/GameModes/BP_TurnBasedGameMode Object Reference"))
  ;[1 1 1] Store controller reference
  (set `local.ControllerReference` Controller)
  ;[1 1 1] If we are not performing an action already
  (if (`|EnumEquality` (`self.ActionState`) "NewEnumerator0")
    ;[1 1 1] Check we are player controlled
    (bind _iscontrolledteam (`self.CheckControlledTeam`))
    (if _iscontrolledteam
      (`|ExecutionSequence`
        (:`then_0`
          ;[1 1 1] Set game mode and participant under cursor
          (bind _participant (`self.CheckValidTargetUnderCursor` (`local.ControllerReference`)))
          (set `local.ParticipantUnderCursor` _participant)
          (bind _gamemode (`self.GetGameMode`))
          (set `local.GameMode` _gamemode)
          ;[1 1 1] Do action depending on menu selection
          (switch `/Game/TurnBasedBattleSystems/Core/Characters/Enumerations/ActionState` (`self.MenuActionState`)
            (:`NewEnumerator1`
              ;[1 1 1] If preselect, set as target, otherwise attack
              (if (`/Game/TurnBasedBattleSystems/Core/GameModes/BP_TurnBasedGameMode.Preselect` (`local.GameMode`))
                (set `self.PreselectTarget` (`local.ParticipantUnderCursor`))
                (set `self.ActionState` "NewEnumerator1")
                (`/Game/TurnBasedBattleSystems/Core/GameModes/BP_TurnBasedGameMode.ParticipantEndAction` (`local.GameMode`) self)
                (`self.ActionSuccessful`)
                (else
                  (`self.MoveToAttack` (`local.ParticipantUnderCursor`))
                  (set `self.ActionState` "NewEnumerator1")
                  (`self.ActionSuccessful`))))
            (:`NewEnumerator2`
              ;[1 1 1] If preselect, set as target, otherwise cast spell
              (if (`/Game/TurnBasedBattleSystems/Core/GameModes/BP_TurnBasedGameMode.Preselect` (`local.GameMode`))
                (set `self.PreselectTarget` (`local.ParticipantUnderCursor`))
                (set `self.ActionState` "NewEnumerator2")
                (`/Game/TurnBasedBattleSystems/Core/GameModes/BP_TurnBasedGameMode.ParticipantEndAction` (`local.GameMode`) self)
                (`self.ActionSuccessful`)
                (else
                  (`self.CastSpellAtTarget` (`local.ParticipantUnderCursor`))
                  (set `self.ActionState` "NewEnumerator2")
                  (`self.ActionSuccessful`))))))
        (:`then_1`
          ;[1 1 1] Remove highlight on targets
          (bind _gamemode_2 (`self.GetGameMode`))
          (for _array_element (`/Game/TurnBasedBattleSystems/Core/GameModes/BP_TurnBasedGameMode.Participants` _gamemode_2)
            (`self.Highlight` _array_element false (struct :`A` 1.0))))))))

(fn `SetColor`
  (params (Value :type "LinearColor Structure"))
  ;[1 1 1] Set the colour of the mannequin body
  (`MaterialInstanceDynamic.SetVectorParameterValue` (`self.CharacterDI`) "BodyColor" Value))

(fn `SetMenuActionState`
  (params (NewState :type "/Game/TurnBasedBattleSystems/Core/Characters/Enumerations/ActionState Enum"))
  (locals (CurrentParticipant :type "/Game/TurnBasedBattleSystems/Core/Characters/BP_Participant Object Reference"))
  ;[1 1 1] Store and switch on the value of menu action state
  (bind _output_get (set `self.MenuActionState` NewState))
  (switch `/Game/TurnBasedBattleSystems/Core/Characters/Enumerations/ActionState` _output_get
    (:`NewEnumerator1`
      _)
    (:`NewEnumerator2`
      _))
  ;[1 1 1] Highlight targets
  (bind _gamemode (`self.GetGameMode`))
  (for _array_element (`/Game/TurnBasedBattleSystems/Core/GameModes/BP_TurnBasedGameMode.Participants` _gamemode)
    (bind _output_get_2 (set `local.CurrentParticipant` _array_element))
    (if (!= (`/Game/TurnBasedBattleSystems/Core/Characters/BP_Participant.Team` _output_get_2) (`self.Team`))
      (`self.Highlight` (`local.CurrentParticipant`) true (struct :`R` 1.0 :`G` 0.772655 :`A` 1.0)))))

(fn `SmoothRotation`
  (params (DeltaTime :type "Float (double-precision)"))
  (locals (DeltaTimeFrame :type "Float (double-precision)"))
  (bind (_returnvalue_roll _returnvalue_pitch _returnvalue_yaw) (`KismetMathLibrary.BreakRotator` (`KismetMathLibrary.NormalizedDeltaRotator` (`self.DesiredRotation`) (`self.K2_GetActorRotation`))))
  ;[1 1 1] Store delta time
  (set `local.DeltaTimeFrame` DeltaTime)
  ;[1 1 1] If smooth rotate flag is set, Interpolate our rotation towards the desired
  (if (`self.SmoothRotate`)
    (`self.K2_SetActorRotation` (`KismetMathLibrary.RInterpTo` (`self.K2_GetActorRotation`) (`self.DesiredRotation`) (`local.DeltaTimeFrame`) 10.0))
    ;[1 1 1] If within a certain tolerance, reset the flag
    (if (`KismetMathLibrary.NearlyEqual_FloatFloat` (`KismetMathLibrary.Abs` _returnvalue_yaw) 0.0 5.0)
      (set `self.SmoothRotate` false))))

(fn `StartTurn`
  ;[1 1 1] Indicate it's our turn
  (`self.FlashTurnMarker`)
  ;[1 1 1] Check participants team
  (bind _iscontrolledteam (`self.CheckControlledTeam`))
  (if _iscontrolledteam
    ;[1 1 1] Participant is player team
    (`self.PlayerControlledAction`)
    (else
      ;[1 1 1] Participant is other team
      (`self.AIControlledAction`))))

(fn `UserConstructionScript`
  (bind _returnvalue (`PrimitiveComponent.CreateDynamicMaterialInstance` (`self.Mesh`) 0 "/Game/TurnBasedBattleSystems/Core/Characters/Mannequin/Character/Materials/M_UE4Man_Body.M_UE4Man_Body"))
  (set `self.CharacterDI` _returnvalue)
  (`self.SetColor` (struct :`A` 1.0))
  (bind _returnvalue_2 (`PrimitiveComponent.CreateDynamicMaterialInstance` (`self.TurnMarker`) 0 "/Game/TurnBasedBattleSystems/MaterialLibrary/Debug/M_BaseColour.M_BaseColour"))
  (bind _output_get (set `self.TurnMarkerDI` _returnvalue_2))
  (`MaterialInstanceDynamic.SetScalarParameterValue` _output_get "Opacity" 0.0)
  (`MaterialInstanceDynamic.SetVectorParameterValue` _output_get "Color" (struct :`R` 0.295268 :`B` 1.0 :`A` 1.0)))