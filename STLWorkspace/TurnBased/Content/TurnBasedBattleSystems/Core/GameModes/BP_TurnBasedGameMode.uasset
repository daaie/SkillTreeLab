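; Base game mode for turn-based battles, managing participants, turn order UI and win/loss.
; BeginPlay adds a dynamic highlight post-process material and shows the game type name.
; StartBattle builds the turn order widgets, then turns chain through ParticipantEndAction and GetNextParticipant, which checks for one remaining team.
; GetNextParticipant selects nobody here; helpers provide wrap-around indexing and widget refresh for sorted participant arrays.
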(event `self.ReceiveBeginPlay`
  ;[1 1 1] Create a dynamic material instance of the highlight material, add it to the blendables of the highlight component
  (bind _returnvalue (`KismetMaterialLibrary.CreateDynamicMaterialInstance` "/Game/TurnBasedBattleSystems/Effects/Materials/M_Highlight_Inst.M_Highlight_Inst"))
  (bind _output_get (set `self.HighlightMaterial` _returnvalue))
  (`PostProcessComponent.AddOrUpdateBlendable` (`self.Highlight`) _output_get 1.0)
  ;[1 1 1] Print the name of the game type
  (bind _returnvalue_2 (`|CreateWidget` "/Game/TurnBasedBattleSystems/UI/WBP_GameTypeText.WBP_GameTypeText_C" null (`self.Name`)))
  (`UserWidget.AddToViewport` _returnvalue_2 0))

(fn `AddParticipant`
  (params (Participant :type "/Game/TurnBasedBattleSystems/Core/Characters/BP_Participant Object Reference"))
  (returns (Successful :type Boolean) (ParticipantIndex :type Integer))
  (locals (NewParticipant :type "/Game/TurnBasedBattleSystems/Core/Characters/BP_Participant Object Reference") (NewParticipantIndex :type Integer))
  ;[1 1 1] Add to turn order if valid
  (bind _output_get (set `local.NewParticipant` Participant))
  (`/Engine/EditorBlueprintResources/StandardMacros.IsValid` _output_get
    (:`Is Valid`
      (`/Game/TurnBasedBattleSystems/Core/Characters/BP_Participant.InitiateCombat` (`local.NewParticipant`))
      (bind _returnvalue (`KismetArrayLibrary.Array_AddUnique` (`self.Participants`) (`local.NewParticipant`)))
      (set `local.NewParticipantIndex` _returnvalue)
      ;[1 0 0.7366] Debug Text
      (if (>= (`local.NewParticipantIndex`) 0)
        (`KismetSystemLibrary.PrintString` (`KismetStringLibrary.Concat_StrStr` (`KismetSystemLibrary.GetObjectName` (`local.NewParticipant`)) " was successfully added to turn order.") false)
        ;[1 1 1] Return participant index successfully
        (return true (`local.NewParticipantIndex`))
        (else
          (`KismetSystemLibrary.PrintString` (`KismetStringLibrary.Concat_StrStr` (`KismetSystemLibrary.GetObjectName` (`local.NewParticipant`)) " already exists in the turn order.") false)
          (return false 0))))
    (:`Is Not Valid`
      ;[1 1 1] Show error message if not valid
      (`KismetSystemLibrary.PrintString` "Participant was not valid!" false)
      (return false 0))))

(fn `CheckVictory`
  (returns (ReturnValue :type Boolean) (Team :type Integer))
  (locals (NoOfTeams :type "Array of Integer"))
  (bind _noofteams (`local.NoOfTeams`))
  (for _array_element (`self.Participants`)
    (`KismetArrayLibrary.Array_AddUnique` (`local.NoOfTeams`) (`/Game/TurnBasedBattleSystems/Core/Characters/BP_Participant.Team` _array_element)))
  ;[1 1 1] If only one team left, return true
  (return (<= (`KismetArrayLibrary.Array_Length` _noofteams) 1) (`KismetArrayLibrary.Array_Get` _noofteams)))

(fn `Defeat`
  ;[1 1 1] Show defeat text
  (`/Game/TurnBasedBattleSystems/Core/Characters/BP_Participant.CreateInfoTextWidget` (`KismetArrayLibrary.Array_Get` (`self.Participants`)) "Enemies Win!")
  ;[1 1 1] End the battle
  (`self.EndBattle`))

(fn `EndBattle`
  ;[1 1 1] Clear array at end of battle
  (`KismetArrayLibrary.Array_Clear` (`self.Participants`)))

(fn `GetNextParticipant`
  (returns (NextParticipant :type "/Game/TurnBasedBattleSystems/Core/Characters/BP_Participant Object Reference"))
  (locals (TeamValue :type Integer) (VictoryResult :type Boolean))
  ;[1 1 1] Check if only one team remains
  (bind (_returnvalue _team) (`self.CheckVictory`))
  (set `local.VictoryResult` _returnvalue)
  (set `local.TeamValue` _team)
  (if (not (`local.VictoryResult`))
    ;[1 1 1] Continue as normal
    (return null)
    (else
      ;[1 1 1] Execute victory/defeat code
      (switch `int` (`local.TeamValue`)
        (:`Default`
          (`self.Victory`))
        (:`0`
          (`self.Victory`))
        (:`1`
          (`self.Defeat`)))
      (return null))))

(fn `GetParticipantFromCurrentIndex`
  (params (ParticipantArray :type "Array of /Game/TurnBasedBattleSystems/Core/Characters/BP_Participant Object Reference (by ref)"))
  (returns (NextParticipant :type "/Game/TurnBasedBattleSystems/Core/Characters/BP_Participant Object Reference"))
  (locals (NewParticipant :type "/Game/TurnBasedBattleSystems/Core/Characters/BP_Participant Object Reference") (ArrayOfSortedParticipants :type "Array of /Game/TurnBasedBattleSystems/Core/Characters/BP_Participant Object Reference"))
  ;[1 1 1] Store sorted array
  (bind _output_get (set `local.ArrayOfSortedParticipants` ParticipantArray))
  ;[1 1 1] Ensure populated array
  (if (> (`KismetArrayLibrary.Array_Length` _output_get) 0)
    ;[1 1 1] Get new participant based on current index
    (set `local.NewParticipant` (`KismetArrayLibrary.Array_Get` (`local.ArrayOfSortedParticipants`) (`self.CurrentParticipantIndex`)) :!label _label)
    ;[1 1 1] Increment current index and ensure it is in array range
    (bind _result (`/Engine/EditorBlueprintResources/StandardMacros.IncrementInt` (`self.CurrentParticipantIndex`))
      (:`  `
        (if (not (not (> _result (`KismetArrayLibrary.Array_LastIndex` (`local.ArrayOfSortedParticipants`)))))
          (set `self.CurrentParticipantIndex` 0))
        (`/Engine/EditorBlueprintResources/StandardMacros.IsValid` (`local.NewParticipant`)
          (:`Is Valid`
            ;[1 1 1] Return new participant
            (return (`local.NewParticipant`)))
          (:`Is Not Valid`
            (goto _label)))))
    (else
      (return null))))

(fn `ParticipantEndAction`
  (params (ParticipantReference :type "/Game/TurnBasedBattleSystems/Core/Characters/BP_Participant Object Reference"))
  ;[1 1 1] Get the next participant and start their turn
  (bind _nextparticipant (`self.GetNextParticipant`))
  (`/Engine/EditorBlueprintResources/StandardMacros.IsValid` _nextparticipant
    (:`Is Valid`
      (bind _output_get (set `self.CurrentParticipant` _nextparticipant))
      (`/Game/TurnBasedBattleSystems/Core/Characters/BP_Participant.StartTurn` _output_get))))

(fn `RemoveParticipant`
  (params (Participant :type "/Game/TurnBasedBattleSystems/Core/Characters/BP_Participant Object Reference"))
  (locals (ParticipantToRemove :type "/Game/TurnBasedBattleSystems/Core/Characters/BP_Participant Object Reference"))
  ;[1 1 1] Check participant is valid
  (bind _output_get (set `local.ParticipantToRemove` Participant))
  (`/Engine/EditorBlueprintResources/StandardMacros.IsValid` _output_get
    (:`Is Valid`
      ;[1 1 1] If not the last participant in the list
      (if (not (not (== (`local.ParticipantToRemove`) (`KismetArrayLibrary.Array_Get` (`self.Participants`)))))
        ;[1 1 1] Decrement counter
        (set `self.CurrentParticipantIndex` (- (`self.CurrentParticipantIndex`) 1)))
      ;[1 1 1] Remove participant
      (bind _returnvalue (`KismetArrayLibrary.Array_RemoveItem` (`self.Participants`) (`local.ParticipantToRemove`)))
      ;[1 0 0.7366] Debug Text
      (if _returnvalue
        (`KismetSystemLibrary.PrintString` (`KismetStringLibrary.Concat_StrStr` (`KismetSystemLibrary.GetObjectName` (`local.ParticipantToRemove`)) " was successfully removed from the turn order.") false)
        (else
          (`KismetSystemLibrary.PrintString` (`KismetStringLibrary.Concat_StrStr` (`KismetSystemLibrary.GetObjectName` (`local.ParticipantToRemove`)) " could not be removed from the turn order.") false))))
    (:`Is Not Valid`
      ;[1 1 1] Show error message
      (`KismetSystemLibrary.PrintString` "Participant was not valid!" false))))

(fn `StartBattle`
  (locals (ParticipantCreatingWidget :type "/Game/TurnBasedBattleSystems/Core/Characters/BP_Participant Object Reference"))
  ;[1 1 1] Create turn order widget
  (bind _returnvalue (`|CreateWidget` "/Game/TurnBasedBattleSystems/UI/WBP_TurnOrder.WBP_TurnOrder_C"))
  (bind _output_get (set `self.TurnOrderWidget` _returnvalue))
  (`UserWidget.AddToViewport` _output_get 0)
  ;[1 1 1] Add counter to turn order
  (for _array_element (`self.Participants`)
    (set `local.ParticipantCreatingWidget` _array_element)
    (bind _returnvalue_2 (`|CreateWidget` "/Game/TurnBasedBattleSystems/UI/WBP_Counter.WBP_Counter_C" null (`local.ParticipantCreatingWidget`) (`self.PreCounterText`)))
    (`HorizontalBox.AddChildToHorizontalBox` (`/Game/TurnBasedBattleSystems/UI/WBP_TurnOrderItem.TurnOrderHorizontalBox` (`/Game/TurnBasedBattleSystems/Core/Characters/BP_Participant.MyTurnOrderWidget` (`local.ParticipantCreatingWidget`))) _returnvalue_2))
  ;[1 1 1] Get next participant, if valid set it as the current participant and start its turn
  (bind _nextparticipant (`self.GetNextParticipant`))
  (`/Engine/EditorBlueprintResources/StandardMacros.IsValid` _nextparticipant
    (:`Is Valid`
      (bind _output_get_2 (set `self.CurrentParticipant` _nextparticipant))
      (`/Game/TurnBasedBattleSystems/Core/Characters/BP_Participant.StartTurn` _output_get_2))))

(fn `UpdateTurnOrderWidget`
  (params (OrderedParticipants :type "Array of /Game/TurnBasedBattleSystems/Core/Characters/BP_Participant Object Reference"))
  (locals (ArrayOfSortedParticipants :type "Array of /Game/TurnBasedBattleSystems/Core/Characters/BP_Participant Object Reference"))
  ;[1 1 1] Clear the widget
  (set `local.ArrayOfSortedParticipants` OrderedParticipants)
  (`PanelWidget.ClearChildren` (`/Game/TurnBasedBattleSystems/UI/WBP_TurnOrder.TurnOrderVerticalBox` (`self.TurnOrderWidget`)))
  ;[1 1 1] Add child for each participant in input array
  (for _array_element (`local.ArrayOfSortedParticipants`)
    (`VerticalBox.AddChildToVerticalBox` (`/Game/TurnBasedBattleSystems/UI/WBP_TurnOrder.TurnOrderVerticalBox` (`self.TurnOrderWidget`)) (`/Game/TurnBasedBattleSystems/Core/Characters/BP_Participant.MyTurnOrderWidget` _array_element))))

(fn `UserConstructionScript`)

(fn `Victory`
  ;[1 1 1] Show victory text
  (`/Game/TurnBasedBattleSystems/Core/Characters/BP_Participant.CreateInfoTextWidget` (`KismetArrayLibrary.Array_Get` (`self.Participants`)) "Players Win!")
  ;[1 1 1] End the battle
  (`self.EndBattle`))