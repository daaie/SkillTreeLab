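; Turn-based battle game mode that adds a preselection scheme on top of agility-ordered turns, alternating between Selection and Action phases.
; Overrides keep an agility-sorted list of pending participants, removing each as it ends its action or leaves battle.
; When the list empties, the mode flips phase, re-sorts, checks victory and shows the phase text.
; In Action phase the next participant runs its preselected action; in Selection phase the parent turn logic runs.
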(event `self.StartBattle`
  ;[1 1 1] Start Battle Override - Sort our initial participants on battle start
  ;;[1 1 1] Override sets sorted and preselection list
  (bind _sortedparticipants (`self.AgilitySort` (`self.Participants`)))
  (bind _output_get (set `self.PreselectionParticipantsList` _sortedparticipants))
  ;;[1 1 1] Show phase widget (selection or action)
  (`/Game/TurnBasedBattleSystems/Core/Characters/BP_Participant.CreateInfoTextWidget` (`KismetArrayLibrary.Array_Get` _output_get) (select `bool` (`self.ActionMode`) :`false` "Selection Phase!" :`true` "Action Phase!"))
  (`parent.StartBattle`))

(event `self.ParticipantEndAction`
  (params (ParticipantReference :type "/Game/TurnBasedBattleSystems/Core/Characters/BP_Participant Object Reference"))
  ;[1 1 1] Participant End Action Override
  ;;[1 1 1] Store the participant calling End Action
  (set `self.ParticipantEndingAction` ParticipantReference)
  ;;[1 1 1] Remove participant from list
  (bind _returnvalue (`KismetArrayLibrary.Array_RemoveItem` (`self.PreselectionParticipantsList`) (`self.ParticipantEndingAction`)))
  (if (not _returnvalue)
    ;;[1 1 1] Print error message
    (`KismetSystemLibrary.PrintString` "Could not remove participant from preselect list!" false))
  ;;[1 1 1] Change to action mode or preselection mode when array is empty
  ;;;[1 1 1] If array is populated
  (if (not (> (`KismetArrayLibrary.Array_Length` (`self.PreselectionParticipantsList`)) 0))
    ;;;[1 1 1] Toggle action mode
    (set `self.ActionMode` (not (`self.ActionMode`)))
    ;;;[1 1 1] Reset list
    (bind _sortedparticipants (`self.AgilitySort` (`self.Participants`)))
    (set `self.PreselectionParticipantsList` _sortedparticipants)
    ;;;[1 1 1] Check victory
    (bind _returnvalue_2 (`self.CheckVictory`))
    (if (not _returnvalue_2)
      ;;[1 1 1] Show action/selection widget
      (`self.ShowActionSelectionText`)))
  ;;[1 1 1] Switch on action mode
  (if (`self.ActionMode`)
    ;;;[1 1 1] Action mode
    (bind _nextparticipant (`self.GetNextParticipant`))
    (`/Engine/EditorBlueprintResources/StandardMacros.IsValid` _nextparticipant
      (:`Is Valid`
        (bind _output_get (set `self.CurrentParticipant` _nextparticipant))
        (`/Game/TurnBasedBattleSystems/Core/Characters/BP_Participant.PreselectedAction` _output_get)))
    (else
      ;;;[1 1 1] Select mode
      (`parent.ParticipantEndAction` (`self.ParticipantEndingAction`)))))

(event `self.RemoveParticipant`
  (params (Participant :type "/Game/TurnBasedBattleSystems/Core/Characters/BP_Participant Object Reference"))
  ;[1 1 1] Remove Participant Override - Remove from preselection list
  (`KismetArrayLibrary.Array_RemoveItem` (`self.PreselectionParticipantsList`) Participant)
  (`parent.RemoveParticipant` Participant))

(fn `AgilitySort`
  (params (Participants :type "Array of /Game/TurnBasedBattleSystems/Core/Characters/BP_Participant Object Reference (by ref)"))
  (returns (SortedParticipants :type "Array of /Game/TurnBasedBattleSystems/Core/Characters/BP_Participant Object Reference"))
  ;[1 1 1] Set our sorted list every agility sort
  (bind _sortedparticipants (`parent.AgilitySort` Participants))
  (bind _output_get (set `self.SortedList` _sortedparticipants))
  (return _output_get))

(fn `GetNextParticipant`
  (returns (NextParticipant :type "/Game/TurnBasedBattleSystems/Core/Characters/BP_Participant Object Reference"))
  (locals (ParentFunctionReturn :type "/Game/TurnBasedBattleSystems/Core/Characters/BP_Participant Object Reference"))
  ;[1 1 1] Parent call to get next agility sorted participant
  (bind _nextparticipant (`parent.GetNextParticipant`))
  (set `local.ParentFunctionReturn` _nextparticipant)
  ;[1 1 1] Update turn order
  (`self.UpdateTurnOrderWidget` (`self.SortedList`))
  (return (`local.ParentFunctionReturn`)))

(fn `ShowActionSelectionText`
  ;[1 1 1] Create info text widget for phase
  (`/Game/TurnBasedBattleSystems/Core/Characters/BP_Participant.CreateInfoTextWidget` (`KismetArrayLibrary.Array_Get` (`self.PreselectionParticipantsList`)) (select `bool` (`self.ActionMode`) :`false` "Selection Phase!" :`true` "Action Phase!")))

(fn `UserConstructionScript`
  (`parent.UserConstructionScript`))