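; Turn-based battle game mode in which all participants first preselect actions in a Selection Phase, then perform them in an Action Phase.
; A working copy of the participant list shrinks as each ends its action or is removed; an action end that empties it flips the phase and resets it.
; Selection turns defer to parent logic, while action turns trigger PreselectedAction on the next participant by index, after the parent's victory check.
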(event `self.StartBattle`
  ;[1 1 1] Start Battle override - Reset widget and set counter values
  (`self.ResetAndShowWidget`)
  (`parent.StartBattle`)
  (for (_array_element _array_index) (`self.Participants`)
    (set `/Game/TurnBasedBattleSystems/Core/Characters/BP_Participant.Counter` _array_index _array_element)))

(event `self.ParticipantEndAction`
  (params (ParticipantReference :type "/Game/TurnBasedBattleSystems/Core/Characters/BP_Participant Object Reference"))
  ;[1 1 1] Participant End Action Override
  ;;[1 1 1] Store participant calling function
  (set `self.ParticipantEndingAction` ParticipantReference)
  ;;[1 1 1] Remove participant from list
  (bind _returnvalue (`KismetArrayLibrary.Array_RemoveItem` (`self.PreselectionParticipantsList`) (`self.ParticipantEndingAction`)))
  (if (not _returnvalue)
    ;;[1 1 1] Show error message
    (`KismetSystemLibrary.PrintString` "Could not remove participant from preselect list!" false))
  ;;[1 1 1] Change to action mode or preselection mode when array is empty
  (if (not (> (`KismetArrayLibrary.Array_Length` (`self.PreselectionParticipantsList`)) 0))
    (set `self.ActionMode` (not (`self.ActionMode`)))
    ;;[1 1 1] Reset the widget
    (`self.ResetAndShowWidget`))
  (if (`self.ActionMode`)
    ;;[1 1 1] Action mode
    (bind _nextparticipant (`self.GetNextParticipant`))
    (`/Engine/EditorBlueprintResources/StandardMacros.IsValid` _nextparticipant
      (:`Is Valid`
        (bind _output_get (set `self.CurrentParticipant` _nextparticipant))
        (`/Game/TurnBasedBattleSystems/Core/Characters/BP_Participant.PreselectedAction` _output_get)))
    (else
      ;;[1 1 1] Select mode
      (`parent.ParticipantEndAction` (`self.ParticipantEndingAction`)))))

(event `self.RemoveParticipant`
  (params (Participant :type "/Game/TurnBasedBattleSystems/Core/Characters/BP_Participant Object Reference"))
  ;[1 1 1] Remove Participant Override - Remove from preselection list
  (set `self.RemovedParticipant` Participant)
  (`KismetArrayLibrary.Array_RemoveItem` (`self.PreselectionParticipantsList`) (`self.RemovedParticipant`))
  (`parent.RemoveParticipant` (`self.RemovedParticipant`)))

(fn `GetNextParticipant`
  (returns (NextParticipant :type "/Game/TurnBasedBattleSystems/Core/Characters/BP_Participant Object Reference"))
  (locals (NextParticipantFromIndex :type "/Game/TurnBasedBattleSystems/Core/Characters/BP_Participant Object Reference"))
  ;[1 1 1] Parent call required for victory check
  (`parent.GetNextParticipant`)
  ;[1 1 1] Get next participant
  (bind _nextparticipant (`self.GetParticipantFromCurrentIndex` (`self.Participants`)))
  (set `local.NextParticipantFromIndex` _nextparticipant)
  ;[1 1 1] Update the turn order widget
  (`self.UpdateTurnOrderWidget` (`self.Participants`))
  ;[1 1 1] Return the next participant
  (return (`local.NextParticipantFromIndex`)))

(fn `ResetAndShowWidget`
  ;[1 1 1] Reset the preselection array
  (set `self.PreselectionParticipantsList` (`self.Participants`))
  ;[1 1 1] Show some text so say which mode we are in
  (bind _returnvalue (`self.CheckVictory`))
  (if (not _returnvalue)
    (`/Game/TurnBasedBattleSystems/Core/Characters/BP_Participant.CreateInfoTextWidget` (`KismetArrayLibrary.Array_Get` (`self.PreselectionParticipantsList`)) (select `bool` (`self.ActionMode`) :`false` "Selection Phase!" :`true` "Action Phase!"))))

(fn `UserConstructionScript`
  (`parent.UserConstructionScript`))