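; Turn-based battle game mode in which participants take turns team by team.
; On battle start it records teams in first-seen order, queues the first team's members and sets each participant's Counter to its team's index.
; GetNextParticipant steps through the current team, skipping invalid or dead members, and GetNextTeam cycles to refill the queue when it runs out.
; Each turn passes a team-sorted participant list to the turn order widget.
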(event `self.StartBattle`
  ;[1 1 1] Start battle override
  ;;[1 1 1] Get an array of teams
  (for _array_element (`self.Participants`)
    (bind _output_get (set `self.CurrentLoopParticipant` _array_element))
    (bind _team (`/Game/TurnBasedBattleSystems/Core/Characters/BP_Participant.Team` _output_get))
    (`KismetArrayLibrary.Array_AddUnique` (`self.Team`) _team)
    ;;[1 1 1] If on the first team added, add this participant to an array
    (if (== _team (`KismetArrayLibrary.Array_Get` (`self.Team`)))
      (`KismetArrayLibrary.Array_Add` (`self.CurrentTeamParticipants`) (`self.CurrentLoopParticipant`))))
  ;;[1 1 1] Call parent function
  (`parent.StartBattle`)
  ;;[1 1 1] Set counter value to order of team added
  (for _array_element_2 (`self.Participants`)
    (set `/Game/TurnBasedBattleSystems/Core/Characters/BP_Participant.Counter` (`KismetArrayLibrary.Array_Find` (`self.Team`) (`/Game/TurnBasedBattleSystems/Core/Characters/BP_Participant.Team` _array_element_2)) _array_element_2)))

(fn `GetNextParticipant`
  (returns (NextParticipant :type "/Game/TurnBasedBattleSystems/Core/Characters/BP_Participant Object Reference"))
  (locals (NewParticipant :type "/Game/TurnBasedBattleSystems/Core/Characters/BP_Participant Object Reference"))
  ;[1 1 1] Parent call for victory check
  (`parent.GetNextParticipant`)
  ;[1 1 1] Get new participant based on current index
  (set `local.NewParticipant` (`KismetArrayLibrary.Array_Get` (`self.CurrentTeamParticipants`) (`self.CurrentParticipantIndex`)) :!label _label)
  ;[1 1 1] Increment current index and ensure it is in array range
  (bind _result (`/Engine/EditorBlueprintResources/StandardMacros.IncrementInt` (`self.CurrentParticipantIndex`))
    (:`  `
      (if (not (not (> _result (`KismetArrayLibrary.Array_LastIndex` (`self.CurrentTeamParticipants`)))))
        ;[1 1 1] Out of range so get next team
        (`self.GetNextTeam`))
      ;[1 1 1] Check our new participant is valid
      (if (and (`KismetSystemLibrary.IsValid` (`local.NewParticipant`)) (not (`/Game/TurnBasedBattleSystems/Core/Characters/BP_Participant.Dead` (`local.NewParticipant`))))
        ;[1 1 1] Update turn order widget
        (bind _sorted (`self.GetTeamSortedParticipants`))
        (`self.UpdateTurnOrderWidget` _sorted)
        ;[1 1 1] Return next participant
        (return (`local.NewParticipant`))
        (else
          (goto _label))))))

(fn `GetNextTeam`
  (locals (ParticipantToTakeTurn :type "/Game/TurnBasedBattleSystems/Core/Characters/BP_Participant Object Reference"))
  ;[1 1 1] Get the next team number based on the turn order index counter
  ;;[1 1 1] Increment and reset if above last index
  (bind _result (`/Engine/EditorBlueprintResources/StandardMacros.IncrementInt` (`self.CurrentTeamIndex`) :!label _label)
    (:`  `
      (if (not (not (> _result (`KismetArrayLibrary.Array_LastIndex` (`self.Team`)))))
        (set `self.CurrentTeamIndex` 0))
      ;;[1 1 1] Clear current array and reset current participant index
      (`KismetArrayLibrary.Array_Clear` (`self.CurrentTeamParticipants`))
      (set `self.CurrentParticipantIndex` 0)
      ;;[1 1 1] If team still exists in array of teams
      (if (>= (`KismetArrayLibrary.Array_Find` (`self.Team`) (`self.CurrentTeamIndex`)) 0)
        ;[1 1 1] Add participants on the team taking their turn to the turn order array
        (for _array_element (`self.Participants`)
          (bind _output_get (set `local.ParticipantToTakeTurn` _array_element))
          (if (== (`/Game/TurnBasedBattleSystems/Core/Characters/BP_Participant.Team` _output_get) (`KismetArrayLibrary.Array_Get` (`self.Team`) (`self.CurrentTeamIndex`)))
            (`KismetArrayLibrary.Array_Add` (`self.CurrentTeamParticipants`) (`local.ParticipantToTakeTurn`))))
        (else
          (goto _label))))))

(fn `GetTeamSortedParticipants`
  (returns (Sorted :type "Array of /Game/TurnBasedBattleSystems/Core/Characters/BP_Participant Object Reference"))
  (locals (SortedArray :type "Array of /Game/TurnBasedBattleSystems/Core/Characters/BP_Participant Object Reference") (CurrentTeam :type Integer))
  ;[1 1 1] Loop through all teams
  (for _array_element (`self.Team`)
    (set `local.CurrentTeam` _array_element)
    ;[1 1 1] If the current participant is on team[current index] add them to the sorted array
    (for _array_element_2 (`self.Participants`)
      (set `self.CurrentLoopParticipant` _array_element_2)
      (if (== (`/Game/TurnBasedBattleSystems/Core/Characters/BP_Participant.Team` _array_element_2) (`local.CurrentTeam`))
        (`KismetArrayLibrary.Array_Add` (`local.SortedArray`) (`self.CurrentLoopParticipant`)))))
  ;[1 1 1] Return sorted array
  (return (`local.SortedArray`)))

(fn `UserConstructionScript`
  (`parent.UserConstructionScript`))