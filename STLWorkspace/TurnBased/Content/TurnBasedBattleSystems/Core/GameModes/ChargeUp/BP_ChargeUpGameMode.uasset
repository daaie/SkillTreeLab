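; Turn-based battle game mode implementing a charge-up turn system, where each participant's charge fills every tick by Agility times delta time.
; Reaching the threshold starts that participant's turn, queues it as charged, and may pause charging depending on Mode and team control.
; Ending an action checks victory or defeat, otherwise resets that charge and selects the next charged player-controlled participant.
; Parent overrides keep the charge array synced with participants and add per-team charge bar widgets.
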(event `self.ReceiveTick`
  (params (DeltaSeconds :type "Float (single-precision)"))
  ;[1 1 1] Charge participants every tick
  (`self.ChargeParticipants`))

(event `self.ParticipantEndAction`
  (params (ParticipantReference :type "/Game/TurnBasedBattleSystems/Core/Characters/BP_Participant Object Reference"))
  ;[1 1 1] Participant End Action Override
  ;;[1 1 1] Store participant calling function
  (set `self.ParticipantEndingAction` ParticipantReference)
  ;;[1 1 1] Check Victory
  (bind (_returnvalue _team) (`self.CheckVictory`))
  (if (not _returnvalue)
    ;;[1 1 1] Remove from charged participants and reset charge to zero
    (`KismetArrayLibrary.Array_RemoveItem` (`self.ChargedParticipants`) (`self.ParticipantEndingAction`))
    (`KismetArrayLibrary.Array_Set` (`self.Charge`) (`KismetArrayLibrary.Array_Find` (`self.Participants`) (`self.ParticipantEndingAction`)) 0.0)
    ;;[1 1 1] Reset pause and current participant
    (set `self.Pause` false)
    (set `self.CurrentParticipant` null)
    ;;[1 1 1] Get next charged participant participant
    (for _array_element (`self.ChargedParticipants`) :!label _label
      (bind _iscontrolledteam (`/Game/TurnBasedBattleSystems/Core/Characters/BP_Participant.CheckControlledTeam` _array_element))
      (if _iscontrolledteam
        (set `self.CurrentParticipant` _array_element)
        ;;[1 1 1] Pause if mode is set to 'wait'
        (set `self.Pause` (`|EnumEquality` (`self.Mode`) "NewEnumerator0"))
        (`self.BreakLoop`)))
    (else
      (switch `int` _team
        (:`Default`
          (`self.Victory`))
        (:`0`
          (`self.Victory`))
        (:`1`
          (`self.Defeat`))))))

(event `BreakLoop`
  ;[1 1 1] Participant End Action Override
  ;;[1 1 1] Get next charged participant participant
  (goto _label :!via `Break`))

(event `self.RemoveParticipant`
  (params (Participant :type "/Game/TurnBasedBattleSystems/Core/Characters/BP_Participant Object Reference"))
  ;[1 1 1] Remove Participant Override - Remove charge from array when removing participant
  (set `self.ParticipanToBeRemoved` Participant)
  (`KismetArrayLibrary.Array_Remove` (`self.Charge`) (`KismetArrayLibrary.Array_Find` (`self.Participants`) (`self.ParticipanToBeRemoved`)))
  (`parent.RemoveParticipant` (`self.ParticipanToBeRemoved`)))

(event `self.StartBattle`
  ;[1 1 1] Start Battle Override - Set pause
  (set `self.Pause` false))

(fn `AddParticipant`
  (params (Participant :type "/Game/TurnBasedBattleSystems/Core/Characters/BP_Participant Object Reference"))
  (returns (Successful :type Boolean) (ParticipantIndex :type Integer))
  (locals (ParticipantCurrentIndex :type Integer) (WasSuccessful :type Boolean :default false) (ParticipantToAdd :type "/Game/TurnBasedBattleSystems/Core/Characters/BP_Participant Object Reference") (ChargeBarWidgetReference :type "/Game/TurnBasedBattleSystems/UI/WBP_ChargeBar Object Reference") (IsControlledTeam :type Boolean))
  ;[1 1 1] Store partipant calling function
  (bind _output_get (set `local.ParticipantToAdd` Participant))
  ;[1 1 1] If added successfully, add to charge list
  (bind (_successful _participantindex) (`parent.AddParticipant` _output_get))
  (set `local.WasSuccessful` _successful)
  (set `local.ParticipantCurrentIndex` _participantindex)
  (`KismetArrayLibrary.Array_Add` (`self.Charge`))
  ;[1 1 1] Create charge bar widget
  (bind _returnvalue (`|CreateWidget` "/Game/TurnBasedBattleSystems/UI/WBP_ChargeBar.WBP_ChargeBar_C" null (`local.ParticipantToAdd`)))
  (set `local.ChargeBarWidgetReference` _returnvalue)
  ;[1 1 1] Add charge bar to left or right side depending on team
  (bind _iscontrolledteam (`/Game/TurnBasedBattleSystems/Core/Characters/BP_Participant.CheckControlledTeam` (`local.ParticipantToAdd`)))
  (set `local.IsControlledTeam` _iscontrolledteam)
  (bind _chargewidget (`self.GetChargeWidget`))
  (`PanelWidget.AddChild` (select `bool` (`local.IsControlledTeam`) :`false` (`/Game/TurnBasedBattleSystems/UI/WBP_ChargeInfo.EnemyChargeVerticalBox` _chargewidget) :`true` (`/Game/TurnBasedBattleSystems/UI/WBP_ChargeInfo.PlayerChargeVerticalBox` _chargewidget)) (`local.ChargeBarWidgetReference`))
  ;[1 1 1] Return index and if adding was a success
  (return (`local.WasSuccessful`) (`local.ParticipantCurrentIndex`)))

(fn `ChargeParticipants`
  (locals (CurrentIndex :type Integer) (CurrentCharge :type "Float (double-precision)") (CurrentChargingParticipant :type "/Game/TurnBasedBattleSystems/Core/Characters/BP_Participant Object Reference"))
  ;[1 1 1] Pause charge
  (if (not (`self.Pause`))
    ;[1 1 1] For each value of charge stored
    (for (_array_element _array_index) (`self.Charge`)
      (set `local.CurrentCharge` _array_element)
      (set `local.CurrentIndex` _array_index)
      ;[1 1 1] If current participant is not charged
      (set `local.CurrentChargingParticipant` (`KismetArrayLibrary.Array_Get` (`self.Participants`) (`local.CurrentIndex`)))
      (if (not (>= (`KismetArrayLibrary.Array_Find` (`self.ChargedParticipants`) (`local.CurrentChargingParticipant`)) 0))
        ;[1 1 1] Set charge to increment by agility x delta time
        (set `local.CurrentCharge` (+ (`local.CurrentCharge`) (* (`/Game/TurnBasedBattleSystems/Core/Characters/BP_Participant.Agility` (`local.CurrentChargingParticipant`)) (`GameplayStatics.GetWorldDeltaSeconds`))))
        (`KismetArrayLibrary.Array_Set` (`self.Charge`) (`local.CurrentIndex`) (`local.CurrentCharge`))
        ;[1 1 1] If our charge is now above required amount and not paused
        (if (and (>= (`local.CurrentCharge`) (`self.SecondsRequiredForTurn`)) (not (`self.Pause`)))
          (`GameplayStatics.PlaySound2D` "/Game/TurnBasedBattleSystems/Audio/Cue/S_Charged_Cue.S_Charged_Cue")
          ;[1 1 1] Start turn and add to charged participants array
          (`/Game/TurnBasedBattleSystems/Core/Characters/BP_Participant.StartTurn` (`local.CurrentChargingParticipant`))
          (`KismetArrayLibrary.Array_Add` (`self.ChargedParticipants`) (`local.CurrentChargingParticipant`))
          ;[1 1 1] If player controlled set as our current participant if there is no current participant
          (bind _iscontrolledteam (`/Game/TurnBasedBattleSystems/Core/Characters/BP_Participant.CheckControlledTeam` (`local.CurrentChargingParticipant`)))
          (if (not (not _iscontrolledteam))
            (`/Engine/EditorBlueprintResources/StandardMacros.IsValid` (`self.CurrentParticipant`)
              (:`Is Valid`
                _)
              (:`Is Not Valid`
                (set `self.CurrentParticipant` (`local.CurrentChargingParticipant`)))))
          (`self.SetPause` (`local.CurrentChargingParticipant`)))))))

(fn `GetChargeWidget`
  (returns (ChargeWidget :type "/Game/TurnBasedBattleSystems/UI/WBP_ChargeInfo Object Reference"))
  ;[1 1 1] If charge widget is valid
  (`/Engine/EditorBlueprintResources/StandardMacros.IsValid` (`self.ChargeWidget`)
    (:`Is Valid`
      _)
    (:`Is Not Valid`
      ;[1 1 1] Not valid so create the widget and return reference
      (bind _returnvalue (`|CreateWidget` "/Game/TurnBasedBattleSystems/UI/WBP_ChargeInfo.WBP_ChargeInfo_C"))
      (bind _output_get (set `self.ChargeWidget` _returnvalue))
      (`UserWidget.AddToViewport` _output_get 0)))
  ;[1 1 1] Return reference
  (return (`self.ChargeWidget`)))

(fn `SetPause`
  (params (ChargedParticipant :type "/Game/TurnBasedBattleSystems/Core/Characters/BP_Participant Object Reference"))
  (locals (ControlledTeam :type Boolean))
  ;[1 1 1] Store if participant is on controlled team
  (bind _iscontrolledteam (`/Game/TurnBasedBattleSystems/Core/Characters/BP_Participant.CheckControlledTeam` ChargedParticipant))
  (set `local.ControlledTeam` _iscontrolledteam)
  ;[1 1 1] Pause
  (if (or (and (not (`local.ControlledTeam`)) (`|EnumEquality` (`self.Mode`) "NewEnumerator1")) (`|EnumEquality` (`self.Mode`) "NewEnumerator0"))
    (set `self.Pause` true)))

(fn `UserConstructionScript`
  (`parent.UserConstructionScript`))