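; Turn-based battle game mode where turn order follows a per-participant countdown.
; GetNextParticipant decrements every participant's Counter until one reaches zero or below, taking the first found on ties.
; When a participant ends its action, its Counter resets to the action cost.
; CountSort insertion-sorts participants by ascending Counter to refresh the turn order widget at battle start and each turn selection.
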(event `self.StartBattle`
  ;[1 1 1] Start Battle Override - Add countdown to turn order widget
  (`parent.StartBattle`)
  ;;[1 1 1] Sort and update turn order based on initial counter values
  (bind _sortedparticipants (`self.CountSort` (`self.Participants`)))
  (`self.UpdateTurnOrderWidget` _sortedparticipants))

(event `self.ParticipantEndAction`
  (params (ParticipantReference :type "/Game/TurnBasedBattleSystems/Core/Characters/BP_Participant Object Reference"))
  ;[1 1 1] Participant End Action Override - Reset counter to action cost
  (set `self.ParticipantEndingAction` ParticipantReference)
  (set `/Game/TurnBasedBattleSystems/Core/Characters/BP_Participant.Counter` (`self.ActionCost`) (`self.ParticipantEndingAction`))
  (`parent.ParticipantEndAction` (`self.ParticipantEndingAction`)))

(fn `CountSort`
  (params (ParticipantsIn :type "Array of /Game/TurnBasedBattleSystems/Core/Characters/BP_Participant Object Reference"))
  (returns (SortedParticipants :type "Array of /Game/TurnBasedBattleSystems/Core/Characters/BP_Participant Object Reference"))
  (locals (ParticipantsList :type "Array of /Game/TurnBasedBattleSystems/Core/Characters/BP_Participant Object Reference") (CurrentSortParticipant :type "/Game/TurnBasedBattleSystems/Core/Characters/BP_Participant Object Reference") (PreviousIndex :type Integer) (CurrentParticipantCounter :type Integer :default 0) (PrevParticipantCounter :type Integer :default 0) (CurrentIndex :type Integer))
  (bind _item (`KismetArrayLibrary.Array_Get` (`local.ParticipantsList`) (`local.CurrentIndex`)))
  (bind _item_2 (`KismetArrayLibrary.Array_Get` (`local.ParticipantsList`) (`local.PreviousIndex`)))
  ;[1 1 1] Loop through from the second participant to the last
  (bind _output_get (set `local.ParticipantsList` ParticipantsIn))
  (for _index (range 1 (`KismetArrayLibrary.Array_Length` _output_get))
    (set `local.CurrentIndex` _index)
    ;[1 1 1] Variables for comparison
    (set `local.CurrentSortParticipant` _item)
    (set `local.CurrentParticipantCounter` (`/Game/TurnBasedBattleSystems/Core/Characters/BP_Participant.Counter` _item))
    (set `local.PreviousIndex` (- (`local.CurrentIndex`) 1))
    (set `local.PrevParticipantCounter` (`/Game/TurnBasedBattleSystems/Core/Characters/BP_Participant.Counter` (`KismetArrayLibrary.Array_Get` (`local.ParticipantsList`) (`local.PreviousIndex`))))
    ;[1 1 1] While our previous index is in array range and the previous participants agility is higher than the current
    (while (and (>= (`local.PreviousIndex`) 0) (> (`local.PrevParticipantCounter`) (`local.CurrentParticipantCounter`)))
      ;[1 1 1] Move the previous participant forward
      (`KismetArrayLibrary.Array_Set` (`local.ParticipantsList`) (+ (`local.PreviousIndex`) 1) (`KismetArrayLibrary.Array_Get` (`local.ParticipantsList`) (`local.PreviousIndex`)) true)
      ;[1 1 1] Decrement previous index
      (set `local.PreviousIndex` (- (`local.PreviousIndex`) 1))
      ;[1 1 1] If new participant is valid, set a new prev agility
      (`/Engine/EditorBlueprintResources/StandardMacros.IsValid` _item_2
        (:`Is Valid`
          (set `local.PrevParticipantCounter` (`/Game/TurnBasedBattleSystems/Core/Characters/BP_Participant.Counter` _item_2)))))
    ;[1 1 1] Move the current participant into new position
    (`KismetArrayLibrary.Array_Set` (`local.ParticipantsList`) (+ (`local.PreviousIndex`) 1) (`local.CurrentSortParticipant`) true))
  ;[1 1 1] Return sorted list
  (return (`local.ParticipantsList`)))

(fn `GetNextParticipant`
  (returns (NextParticipant :type "/Game/TurnBasedBattleSystems/Core/Characters/BP_Participant Object Reference"))
  (locals (CountDown :type Boolean :default true) (NewParticipant :type "/Game/TurnBasedBattleSystems/Core/Characters/BP_Participant Object Reference") (CurrentLoopParticipant :type "/Game/TurnBasedBattleSystems/Core/Characters/BP_Participant Object Reference"))
  ;[1 1 1] Returns the first participant to have their counter value drop to zero or below (only drops below zero in event of a tie)
  ;;[1 1 1] Parent call for victory check
  (`parent.GetNextParticipant`)
  ;;[1 1 1] While participants is populated and no participant counter is at or below zero (count down flag)
  (while (and (`local.CountDown`) (> (`KismetArrayLibrary.Array_Length` (`self.Participants`)) 0))
    ;;[1 1 1] For each participant
    (for _array_element (`self.Participants`)
      (set `local.CurrentLoopParticipant` _array_element)
      ;;[1 1 1] Decrement counter
      (bind _output_get (set `/Game/TurnBasedBattleSystems/Core/Characters/BP_Participant.Counter` (- (`/Game/TurnBasedBattleSystems/Core/Characters/BP_Participant.Counter` (`local.CurrentLoopParticipant`)) 1) (`local.CurrentLoopParticipant`)))
      ;;[1 1 1] If below or equal zero
      (if (<= _output_get 0)
        ;;[1 1 1] Set count down flag
        (set `local.CountDown` false)
        ;;[1 1 1] If we don't have a participant already in this loop, set as new participant
        (if (not (`KismetSystemLibrary.IsValid` (`local.NewParticipant`)))
          (set `local.NewParticipant` (`local.CurrentLoopParticipant`))))))
  ;;[1 1 1] Sort and update widget
  (bind _sortedparticipants (`self.CountSort` (`self.Participants`)))
  (`self.UpdateTurnOrderWidget` _sortedparticipants)
  (return (`local.NewParticipant`)))

(fn `UserConstructionScript`
  (`parent.UserConstructionScript`))