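; Player-controlled P-38 plane pawn that steers, strafes and fires rockets.
; Tick spins both propellers through a RotateProp custom event and calls forward AddMovementInput, though its scale is zero.
; Axis inputs apply frame-rate-scaled local roll, pitch and sideways offset, while the fire action spawns BP_RocketActor at the Arrow component's transform.
; The forward/back axis is empty, and alternative forward-movement nodes are left disconnected.
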(event `self.ReceiveBeginPlay`)

(event `self.ReceiveTick`
  (params (DeltaSeconds :type "Float (single-precision)"))
  ;[1 1 1] 비행기 이동 및 프로펠러 회전
  (`self.RotateProp` (`self.LProp`))
  (`self.RotateProp` (`self.RProp`))
  (`self.AddMovementInput` (`KismetMathLibrary.GetForwardVector` (`self.K2_GetActorRotation`)) 0.0))

(event `RotateProp`
  (params (Component :type "StaticMeshComponent Object Reference"))
  ;[1 1 1] custom event 는 리플리케이션이 됨..함수는 안됨 네트워크하려면 이거해야함..? custom event는 반환값이 없다
  (`SceneComponent.K2_AddLocalRotation` Component (`KismetMathLibrary.MakeRotator` (* (`self.프로펠러`) (`GameplayStatics.GetWorldDeltaSeconds`))) false false))

(event `InputAxis|앞뒤이동`
  (params (AxisValue :type "Float (single-precision)"))
  ;[1 1 1] 무조건앞으로갈거라고...주석
)

(event `InputAxis|좌우회전`
  (params (AxisValue :type "Float (single-precision)"))
  ;[1 1 1] 비행기 회전 이동
  ;;[1 1 1] 축입력받기
  (`self.K2_AddActorLocalRotation` (`KismetMathLibrary.MakeRotator` (* AxisValue (`GameplayStatics.GetWorldDeltaSeconds`) (`self.회전속도`)))))

(event `InputAction|발사`
  (params (Key :type "Key Structure"))
  ;[1 1 1] 미사일 발사
  (:`Pressed`
    ;;[1 1 1] 생성은 spawn/ owner은 누가 생성하냐 설정 안해주면 자기자신 actor, instigator은 플레이어 설정임(ㄷ데미지 유저정보등?)
    (`|SpawnActorFromClass` "/Game/BluePrint/BP_RocketActor.BP_RocketActor_C" (`SceneComponent.K2_GetComponentToWorld` (`self.Arrow`)) "Undefined" "OverrideRootScale" null null)))

(event `InputAxis|앞회전`
  (params (AxisValue :type "Float (single-precision)"))
  ;[1 1 1] 비행기 회전 이동
  ;;[1 1 1] 축입력받기
  (`self.K2_AddActorLocalRotation` (`KismetMathLibrary.MakeRotator` 0.0 (* AxisValue (`GameplayStatics.GetWorldDeltaSeconds`) (`self.회전속도`)))))

(event `InputAxis|좌우이동`
  (params (AxisValue :type "Float (single-precision)"))
  ;[1 1 1] 비행기 회전 이동
  ;;[1 1 1] 축입력받기
  (`self.K2_AddActorLocalOffset` (`KismetMathLibrary.MakeVector` 0.0 (* AxisValue (`self.이동속도`) (`GameplayStatics.GetWorldDeltaSeconds`)))))

(fn `UserConstructionScript`)