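; BP_P38Actor is an Actor for a P-38 aircraft that spins its left and right propellers.
; Each Tick calls the RotateProp custom event on LProp and RProp, adding local roll scaled by GVelocity and delta seconds.
; A left/right input axis handler only prints its value, and a note says input does not work because the parent class is Actor.
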(event `RotateProp`
  (params (Component :type "StaticMeshComponent Object Reference"))
  ;[1 1 1] custom event 는 리플리케이션이 됨..함수는 안됨 네트워크하려면 이거해야함..? custom event는 반환값이 없다
  (`SceneComponent.K2_AddLocalRotation` Component (`KismetMathLibrary.MakeRotator` (* (`self.G_velocity`) (`GameplayStatics.GetWorldDeltaSeconds`))) false false))

(event `self.ReceiveTick`
  (params (DeltaSeconds :type "Float (single-precision)"))
  (`self.RotateProp` (`self.LProp`))
  (`self.RotateProp` (`self.RProp`)))

(event `InputAxis|좌우이동`
  (params (AxisValue :type "Float (single-precision)"))
  ;[1 1 1] 부모클래스가 엑터라서 입력핸들러가안됨
  (`KismetSystemLibrary.PrintString` (`KismetStringLibrary.Conv_DoubleToString` AxisValue)))

(fn `UserConstructionScript`)