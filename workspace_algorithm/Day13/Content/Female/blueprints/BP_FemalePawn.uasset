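; BP_FemalePawn is a player-controlled female character driven by input events for movement, camera and actions.
; Movement follows control yaw, and Dash toggles walk speed between slow and fast.
; Look input drives controller rotation, with LookUp also shifting the camera vertically, while Zoom changes spring arm length without clamping.
; Jump, Dance and Attack set state flags, of which only IsJump is cleared here.
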(event `InputAction|Dash`
  (params (Key :type "Key Structure"))
  (:`Pressed`
    (if (> (`CharacterMovementComponent.MaxWalkSpeed` (`self.CharacterMovement`)) 300.0)
      (set `CharacterMovementComponent.MaxWalkSpeed` 300.0 (`self.CharacterMovement`))
      (else
        (set `CharacterMovementComponent.MaxWalkSpeed` 600.0 (`self.CharacterMovement`))))))

(event `InputAxis|Zoom`
  (params (AxisValue :type "Float (single-precision)"))
  (set `SpringArmComponent.TargetArmLength` (+ (`SpringArmComponent.TargetArmLength` (`self.SpringArm`)) (* AxisValue 50.0)) (`self.SpringArm`)))

(event `InputAction|Dance`
  (params (Key :type "Key Structure"))
  (:`Pressed`
    (set `self.IsDance` true)))

(event `InputAction|Attack`
  (params (Key :type "Key Structure"))
  (:`Pressed`
    (set `self.IsAttack` true)))

(event `InputAxis|Turn`
  (params (AxisValue :type "Float (single-precision)"))
  (`self.AddControllerYawInput` AxisValue))

(event `InputAxis|MoveForward`
  (params (AxisValue :type "Float (single-precision)"))
  (bind (_returnvalue_roll _returnvalue_pitch _returnvalue_yaw) (`KismetMathLibrary.BreakRotator` (`self.GetControlRotation`)))
  (`self.AddMovementInput` (`KismetMathLibrary.GetForwardVector` (`KismetMathLibrary.MakeRotator` 0.0 0.0 _returnvalue_yaw)) AxisValue))

(event `InputAxis|LookUp`
  (params (AxisValue :type "Float (single-precision)"))
  (`self.AddControllerPitchInput` AxisValue)
  (`SceneComponent.K2_AddLocalOffset` (`self.Camera`) (`KismetMathLibrary.MakeVector` 0.0 0.0 AxisValue) false false))

(event `InputAction|Jump`
  (params (Key :type "Key Structure"))
  (:`Pressed`
    (`self.Jump`)
    (set `self.IsJump` true))
  (:`Released`
    (`self.StopJumping`)
    (set `self.IsJump` false)))

(event `InputAxis|MoveRight`
  (params (AxisValue :type "Float (single-precision)"))
  (bind (_returnvalue_roll _returnvalue_pitch _returnvalue_yaw) (`KismetMathLibrary.BreakRotator` (`self.GetControlRotation`)))
  (`self.AddMovementInput` (`KismetMathLibrary.GetRightVector` (`KismetMathLibrary.MakeRotator` 0.0 0.0 _returnvalue_yaw)) AxisValue))

(fn `UserConstructionScript`)