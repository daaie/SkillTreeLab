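; BP_P38Actor is a P-38 plane actor with spinning left and right propellers that shifts sideways on A and D key presses.
; Tick calls the shared 프로펠러회전 function for each propeller, applying the 회전속도 rotation rate scaled by delta seconds for frame-rate independence.
; Each key press adds a fixed, unswept world Y offset.
; Unconnected leftovers hold an inline rotation version, a summation loop and a counter print.
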(event `self.ReceiveTick`
  (params (DeltaSeconds :type "Float (single-precision)"))
  (`self.프로펠러회전` (`self.왼쪽`))
  (`self.프로펠러회전` (`self.오른쪽`)))

(event `Key|A`
  (params (Key :type "Key Structure"))
  (:`Pressed`
    (`self.K2_AddActorWorldOffset` (0.0 -10.0 0.0))))

(event `Key|D`
  (params (Key :type "Key Structure"))
  (:`Pressed`
    (`self.K2_AddActorWorldOffset` (0.0 10.0 0.0))))

(fn `UserConstructionScript`)

(fn `프로펠러회전`
  (params (`회전컴포넌트` :type "StaticMeshComponent Object Reference"))
  (`SceneComponent.K2_AddLocalRotation` `회전컴포넌트` (* (`self.회전속도`) (`GameplayStatics.GetWorldDeltaSeconds`)) false false))