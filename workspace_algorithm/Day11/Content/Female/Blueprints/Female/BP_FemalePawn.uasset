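; BP_FemalePawn is a player-controlled female character with input for running, jumping, attacking and camera control.
; Movement follows the controller's yaw only, so a tilted camera does not push it toward the ground, and stops while IsAttack is set.
; Run swaps the max walk speed, Turn and LookUp drive controller rotation, and Zoom changes spring arm length without clamping.
; Fire sets IsAttack, and this graph never clears it.
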(event `self.ReceiveBeginPlay`
  (set `self.WalkSpeed` (`CharacterMovementComponent.MaxWalkSpeed` (`self.CharacterMovement`))))

(event `InputAction|Run`
  (params (Key :type "Key Structure"))
  (:`Pressed`
    (set `CharacterMovementComponent.MaxWalkSpeed` (`self.RunSpeed`) (`self.CharacterMovement`)))
  (:`Released`
    (set `CharacterMovementComponent.MaxWalkSpeed` (`self.WalkSpeed`) (`self.CharacterMovement`))))

(event `InputAction|Jump`
  (params (Key :type "Key Structure"))
  (:`Pressed`
    (`self.Jump`)
    (set `self.IsJumping` true))
  (:`Released`
    (`self.StopJumping`)
    (set `self.IsJumping` false)))

(event `InputAction|Fire`
  (params (Key :type "Key Structure"))
  (:`Pressed`
    (set `self.IsAttack` true)))

(event `InputAxis|MoveForward`
  (params (AxisValue :type "Float (single-precision)"))
  ;[1 1 1] movement는 CharacterMovement가 한다..ㅋㅋㅋㅋ자꾸 오프셋하지마ㅜ&ㅜ
  (if (not (`self.IsAttack`))
    (`self.AddMovementInput` (`KismetMathLibrary.GetForwardVector` (`KismetMathLibrary.MakeRotator` 0.0 0.0 (.yaw (`self.GetControlRotation`)))) AxisValue)))

(event `InputAxis|MoveRight`
  (params (AxisValue :type "Float (single-precision)"))
  (if (not (`self.IsAttack`))
    ;[1 1 1] CharacterMovement 기준으로 돌꺼야 pawn Controll이 아니라
    (`self.AddMovementInput` (`KismetMathLibrary.GetRightVector` (`KismetMathLibrary.MakeRotator` 0.0 0.0 (.yaw (`self.GetControlRotation`)))) AxisValue)))

(event `InputAxis|Turn`
  (params (AxisValue :type "Float (single-precision)"))
  ;[1 1 1] Add Controller Yaw는 pawn이 관리하는애 , 이걸쓰려면 pawn self랑 카메라에 Pawn Controll rotation체크해야함
  (`self.AddControllerYawInput` AxisValue))

(event `InputAxis|LookUp`
  (params (AxisValue :type "Float (single-precision)"))
  ;[1 1 1] Add Controller Yaw는 pawn이 관리하는애 , 이걸쓰려면 pawn self랑 카메라에 Pawn Controll rotation체크해야함
  (`self.AddControllerPitchInput` AxisValue))

(event `InputAxis|Zoom`
  (params (AxisValue :type "Float (single-precision)"))
  (set `SpringArmComponent.TargetArmLength` (+ AxisValue (`SpringArmComponent.TargetArmLength` (`self.SpringArm`)) 0.0) (`self.SpringArm`)))

(fn `UserConstructionScript`)