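; Rocket projectile actor that explodes when its Box overlaps any actor not tagged Player.
; The overlap plays an attached collapse sound, spawns an explosion emitter at the rocket's transform and destroys the actor.
; BeginPlay sets a timer on the Destroy event with zero time, so the three-second self-destruct described in its note is not scheduled.
; Delay, named-timer (DestroyRocket) and attached-emitter alternatives remain as unconnected nodes.
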(event `Destroy`
  ;[1 1 1] 3초뒤에 custom event 호출
  (`self.K2_DestroyActor`))

(event `self.ReceiveTick`
  (params (DeltaSeconds :type "Float (single-precision)")))

(event `self.ReceiveBeginPlay`
  ;[1 1 1] 3초뒤에 펑션호출 Looping 체크는 3초에 한번 무조건 실행함
  ;[1 1 1] 3초뒤에 custom event 호출
  (`KismetSystemLibrary.K2_SetTimerDelegate` (delegate `Destroy`)))

(event `self.Box.OnComponentBeginOverlap`
  (params (OverlappedComponent :type "PrimitiveComponent Object Reference") (OtherActor :type "Actor Object Reference") (OtherComp :type "PrimitiveComponent Object Reference") (OtherBodyIndex :type Integer) (bFromSweep :type Boolean) (SweepResult :type "HitResult Structure (by ref)"))
  ;[1 1 1] 겹치기 시작 원래 히트로 처리하는게 맞음
  ;[1 1 1] 충돌시 사라지는거
  (if (not (`self.ActorHasTag` OtherActor "Player"))
    (`GameplayStatics.SpawnSoundAttached` "/Game/StarterContent/Audio/Collapse_Cue.Collapse_Cue" (`self.Box`))
    ;;[1 1 1] location은 위치에
    (`GameplayStatics.SpawnEmitterAtLocation` "/Game/StarterContent/Particles/P_Explosion.P_Explosion" (`self.K2_GetActorLocation`) (`self.K2_GetActorRotation`))
    (`self.K2_DestroyActor`)))

(event `self.Box.OnComponentEndOverlap`
  (params (OverlappedComponent :type "PrimitiveComponent Object Reference") (OtherActor :type "Actor Object Reference") (OtherComp :type "PrimitiveComponent Object Reference") (OtherBodyIndex :type Integer))
  ;[1 1 1] 겹치기 끝
)

(fn `DestroyRocket`
  (`self.K2_DestroyActor`))

(fn `UserConstructionScript`)