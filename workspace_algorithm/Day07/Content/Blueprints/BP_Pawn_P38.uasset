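; BP_Pawn_P38 is a player-controlled plane pawn that flies forward constantly, steers, boosts and fires rockets.
; Tick spins the Left and Right propellers and feeds forward movement input, scaled by a speed variable, to the movement component.
; Roll and pitch axes rotate the actor locally; the booster raises that scale while held and spawns a steam effect on press.
; Fire spawns a Rocket at an arrow component, and Box hits print the other actor's name.
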(event `MakeRotation`
  (params (Component :type "StaticMeshComponent Object Reference"))
  (`SceneComponent.K2_AddLocalRotation` Component (`KismetMathLibrary.MakeRotator` (* (`self.프로펠러속도`) (`GameplayStatics.GetWorldDeltaSeconds`))) false false))

(event `self.ReceiveTick`
  (params (DeltaSeconds :type "Float (single-precision)"))
  (`|ExecutionSequence`
    (:`then_0`
      (`self.MakeRotation` (`self.Left`)))
    (:`then_1`
      (`self.MakeRotation` (`self.Right`)))
    (:`then_2`
      ;[1 1 1] 얘는 FloatingPawnMovement가 움직이는데 여기에 벡터랑 속도비율을 주는것
      (`self.AddMovementInput` (`self.GetActorForwardVector`) (`self.이동속도`)))))

(event `InputAxis|Rolling`
  (params (AxisValue :type "Float (single-precision)"))
  (`self.K2_AddActorLocalRotation` (`KismetMathLibrary.MakeRotator` (* AxisValue (`GameplayStatics.GetWorldDeltaSeconds`) (`self.회전속도`)))))

(event `InputAction|부스터`
  (params (Key :type "Key Structure"))
  ;[1 1 1] 얘는 FloatingPawnMovement가 움직이는데 여기에 벡터랑 속도비율을 주는것
  ;;[1 1 1] 이동속도는 0~1임 속도를 올리고 싶으면 movement의 max값을 올려야한다 가속도, de가속도 조절 가능함
  (:`Pressed`
    (set `self.이동속도` 1.0)
    (`GameplayStatics.SpawnEmitterAtLocation` "/Game/StarterContent/Particles/P_Steam_Lit.P_Steam_Lit" (`SceneComponent.K2_GetComponentLocation` (`self.Arrow1`)) (struct) (3.0 3.0 3.0)))
  (:`Released`
    (set `self.이동속도` 0.5)))

(event `InputAxis|Fitch`
  (params (AxisValue :type "Float (single-precision)"))
  (`self.K2_AddActorLocalRotation` (`KismetMathLibrary.MakeRotator` 0.0 (* AxisValue (`GameplayStatics.GetWorldDeltaSeconds`) (`self.회전속도`)))))

(event `self.Box.OnComponentHit`
  (params (HitComponent :type "PrimitiveComponent Object Reference") (OtherActor :type "Actor Object Reference") (OtherComp :type "PrimitiveComponent Object Reference") (NormalImpulse :type "Vector Structure") (Hit :type "HitResult Structure (by ref)"))
  (`KismetSystemLibrary.PrintString` (`KismetSystemLibrary.GetDisplayName` OtherActor)))

(event `InputAction|발사`
  (params (Key :type "Key Structure"))
  (:`Pressed`
    ;[1 1 1] owner는 컨트롤러...만약 둘이 싸우다 한명이 3대맞춰도 그사이에 헤드샷당하면 총알다날라감.. 소유주가 날라가서
    (`|SpawnActorFromClass` "/Game/Blueprints/Rocket.Rocket_C" (`SceneComponent.K2_GetComponentToWorld` (`self.Arrow`)) "AlwaysSpawn" "OverrideRootScale" null null)))

(fn `UserConstructionScript`)