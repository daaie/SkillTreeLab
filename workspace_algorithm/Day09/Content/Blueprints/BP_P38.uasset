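; BP_P38 is a player-controlled aircraft pawn that constantly flies forward, steers by roll and pitch, and fires rockets.
; Tick spins the Left and Right propellers through a shared function and feeds forward movement input scaled by a speed variable, which the booster action raises while held.
; Axis inputs apply frame-rate-independent local rotations to the actor.
; The fire action spawns BP_Rocket at the Arrow component's transform.
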(event `InputAction|발사`
  (params (Key :type "Key Structure"))
  (:`Pressed`
    (`|SpawnActorFromClass` "/Game/Blueprints/BP_Rocket.BP_Rocket_C" (`SceneComponent.K2_GetComponentToWorld` (`self.Arrow`)) "Undefined" "OverrideRootScale" null null)))

(event `InputAxis|Rolling`
  (params (AxisValue :type "Float (single-precision)"))
  (`self.K2_AddActorLocalRotation` (`KismetMathLibrary.MakeRotator` (* (`self.회전속도`) (`GameplayStatics.GetWorldDeltaSeconds`) AxisValue))))

(event `InputAxis|Pitch`
  (params (AxisValue :type "Float (single-precision)"))
  (`self.K2_AddActorLocalRotation` (`KismetMathLibrary.MakeRotator` 0.0 (* (`self.회전속도`) (`GameplayStatics.GetWorldDeltaSeconds`) AxisValue) 0.0)))

(event `self.ReceiveTick`
  (params (DeltaSeconds :type "Float (single-precision)"))
  (`self.NewFunction_0` (`self.Left`))
  (`self.NewFunction_0` (`self.Right`))
  (`self.AddMovementInput` (`self.GetActorForwardVector`) (`self.이동속도`)))

(event `InputAction|부스터`
  (params (Key :type "Key Structure"))
  (:`Pressed`
    (set `self.이동속도` 1.0))
  (:`Released`
    (set `self.이동속도` 0.5)))

(fn `NewFunction_0`
  (params (Component :type "StaticMeshComponent Object Reference"))
  (`SceneComponent.K2_AddLocalRotation` Component (`KismetMathLibrary.MakeRotator` (* (`self.프로펠러속도`) (`GameplayStatics.GetWorldDeltaSeconds`))) false false))

(fn `UserConstructionScript`)