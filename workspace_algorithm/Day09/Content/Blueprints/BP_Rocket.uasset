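; BP_Rocket is a rocket actor that explodes when its Box component begins overlapping something.
; The overlap plays a collapse sound at the box, spawns a scaled-up explosion emitter at the actor and destroys it, with no filter on what it hit.
; A timer started on BeginPlay destroys the rocket silently after a few seconds if nothing is hit.
; Leftover trace, Player-tag and delay nodes are unconnected.
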(event `self.ReceiveBeginPlay`
  (`KismetSystemLibrary.K2_SetTimerDelegate` (delegate `destroy`) 3.0))

(event `destroy`
  (`self.K2_DestroyActor`))

(event `self.ReceiveActorBeginOverlap`
  (params (OtherActor :type "Actor Object Reference")))

(event `self.Box.OnComponentBeginOverlap`
  (params (OverlappedComponent :type "PrimitiveComponent Object Reference") (OtherActor :type "Actor Object Reference") (OtherComp :type "PrimitiveComponent Object Reference") (OtherBodyIndex :type Integer) (bFromSweep :type Boolean) (SweepResult :type "HitResult Structure (by ref)"))
  (`GameplayStatics.SpawnSoundAtLocation` "/Game/StarterContent/Audio/Collapse_Cue.Collapse_Cue" (`SceneComponent.K2_GetComponentLocation` (`self.Box`)))
  (`GameplayStatics.SpawnEmitterAtLocation` "/Game/StarterContent/Particles/P_Explosion.P_Explosion" (`self.K2_GetActorLocation`) (struct) (3.0 3.0 3.0))
  (`self.K2_DestroyActor`))

(fn `UserConstructionScript`)