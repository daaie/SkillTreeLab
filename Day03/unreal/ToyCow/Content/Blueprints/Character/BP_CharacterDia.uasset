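; BP_CharacterDia is a player character Blueprint with movement, jump, a combo attack and a cooldown-gated skill.
; Tick builds control rotation from the movement axes and moves along the controller's forward vector while input is non-zero.
; Attacks play a montage or pick the next combo section from the current one, with a separate impulse-based dash event.
; A state enum blocks skills during actions, and BP_CharacterController handles skill cooldown.
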(event `InputAxis|Turn`
  (params (AxisValue :type "Float (single-precision)"))
  ;[1 1 1] [회전] - controller z축 회전
)

(event `InputAction|Jump`
  (params (Key :type "Key Structure"))
  (:`Pressed`
    (`self.Jump`)))

(event `InputAxis|LookUp`
  (params (AxisValue :type "Float (single-precision)")))

(event `DoAttack`
  ;[1 1 1] 공격전환
  (set `self.StateBP` "NewEnumerator1" :!label _label)
  (if (`AnimInstance.Montage_IsPlaying` (`SkeletalMeshComponent.GetAnimInstance` (`self.Mesh`)) null)
    (switch `name` (`AnimInstance.Montage_GetCurrentSection` (`SkeletalMeshComponent.GetAnimInstance` (`self.Mesh`)) null)
      (:`Default`
        (set `self.NextSection` "None"))
      (:`Attack1`
        (set `self.NextSection` "Attack2"))
      (:`Attack2`
        (set `self.NextSection` "Attack3"))
      (:`Attack3`
        (set `self.NextSection` "Attack4")))
    (else
      ;[1 1 1] 무조건 몽타주 처음
      (`AnimInstance.Montage_Play` (`SkeletalMeshComponent.GetAnimInstance` (`self.Mesh`)) null 1.0 "MontageLength" 0.0 true))))

(event `InputAction|Attack`
  (params (Key :type "Key Structure"))
  ;[1 1 1] 공격전환
  (:`Pressed`
    (goto _label)))

(event `self.ReceiveTick`
  (params (DeltaSeconds :type "Float (single-precision)"))
  ;[1 1 1] 캐릭터 이동
  (if (or (!= (`self.GetInputAxisValue`) 0.0) (!= (`self.GetInputAxisValue`) 0.0))
    (`Controller.SetControlRotation` (`GameplayStatics.GetPlayerController` 0) (`KismetMathLibrary.MakeRotFromX` (`KismetMathLibrary.MakeVector` (`self.GetInputAxisValue`) (`self.GetInputAxisValue`))))
    (`self.AddMovementInput` (`self.GetActorForwardVector` (`GameplayStatics.GetPlayerController` 0)))))

(event `AttackEnd`
  (set `self.StateBP` "NewEnumerator0"))

(event `self.ReceiveBeginPlay`
  (bind _asbp_character_controller (cast `/Game/Blueprints/Character/BP_CharacterController` (`GameplayStatics.GetPlayerController` 0)))
  (set `self.RefController` _asbp_character_controller))

(event `AttackDash`
  ;[1 1 1] Dash Move
  (`CharacterMovementComponent.AddImpulse` (`self.CharacterMovement`) (* (`self.GetActorForwardVector`) (`self.DashForce`)) true))

(event `DoSkill`
  ;[1 1 1] 스킬
  (bind _canskill (`/Game/Blueprints/Character/BP_CharacterController.CanUseSkill` (`self.RefController`)))
  (if (and _canskill (`|EnumEquality` (`self.StateBP`) "NewEnumerator0"))
    (set `self.StateBP` "NewEnumerator1")
    (`self.PlayAnimMontage` null 1.0 "Skill")
    (`/Game/Blueprints/Character/BP_CharacterController.StartSkillCoolDown` (`self.RefController`))))

(event `SkillEnd`
  (set `self.StateBP` "NewEnumerator0"))

(fn `UserConstructionScript`)