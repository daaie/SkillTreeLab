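; BP_CharacterGTA is a player character with camera-relative movement, look, jump and a basic attack.
; Axis inputs drive controller yaw and pitch, and movement follows the control rotation's forward and right vectors.
; A StateBP enum gates the attack: input switches state and calls PlayAnimMontage at the "Attack" section, and AttackEnd resets it.
; Damage calls are unconnected, and the capsule hit event is empty.
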(event `self.ReceiveBeginPlay`)

(event `InputAction|Jump`
  (params (Key :type "Key Structure"))
  (:`Pressed`
    (`self.Jump`)))

(event `InputAxis|Turn`
  (params (AxisValue :type "Float (single-precision)"))
  ;[1 1 1] [회전] - controller z축 회전
  (`self.AddControllerYawInput` AxisValue))

(event `InputAxis|UpDown`
  (params (AxisValue :type "Float (single-precision)"))
  (`self.AddMovementInput` (`KismetMathLibrary.GetForwardVector` (`self.GetControlRotation`)) AxisValue))

(event `InputAxis|LookUp`
  (params (AxisValue :type "Float (single-precision)"))
  (`self.AddControllerPitchInput` AxisValue))

(event `InputAction|Attack`
  (params (Key :type "Key Structure"))
  ;[1 1 1] 공격전환
  (:`Pressed`
    (if (`|EnumEquality` (`self.StateBP`) "NewEnumerator0")
      (set `self.StateBP` "NewEnumerator1")
      (`self.PlayAnimMontage` null 1.0 "Attack")
      (`KismetSystemLibrary.PrintString` (`|GetEnumeratorNameAsString` (`self.StateBP`))))))

(event `self.CapsuleComponent.OnComponentHit`
  (params (HitComponent :type "PrimitiveComponent Object Reference") (OtherActor :type "Actor Object Reference") (OtherComp :type "PrimitiveComponent Object Reference") (NormalImpulse :type "Vector Structure") (Hit :type "HitResult Structure (by ref)")))

(event `InputAxis|LeftRight`
  (params (AxisValue :type "Float (single-precision)"))
  (`self.AddMovementInput` (`KismetMathLibrary.GetRightVector` (`self.GetControlRotation`)) AxisValue))

(event `AttackEnd`
  (set `self.StateBP` "NewEnumerator0"))

(fn `UserConstructionScript`)