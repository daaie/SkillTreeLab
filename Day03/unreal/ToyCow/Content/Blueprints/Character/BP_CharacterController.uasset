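; Character controller Blueprint that creates the main HUD widget and manages the cooldown of a single skill.
; CanUseSkill reports readiness, and StartSkillCoolDown raises the cooldown flag and fills the HUD indicator.
; Each Tick advances BPTimer toward SkillTime, driving the indicator's dynamic material Percent parameter with the remaining fraction.
; On timeout it resets the timer, clears the flag and sets the indicator to HitTestInvisible; the node setting it Visible is unconnected.
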(event `self.ReceiveBeginPlay`
  ;[1 1 1] texture
  (bind _returnvalue (`|CreateWidget` "/Game/UI/UMG_Main.UMG_Main_C"))
  (bind _output_get (set `self.MainUI` _returnvalue))
  ;[1 1 1] 랜더타겟에
  (`UserWidget.AddToViewport` _output_get 0))

(event `self.ReceiveTick`
  (params (DeltaSeconds :type "Float (single-precision)"))
  (`self.SkillCoolDown`))

(fn `CanUseSkill`
  (returns (CanSkill :type Boolean))
  (return (not (`self.IsSkillCoolDown`))))

(fn `SkillCoolDown`
  (bind _skilltime (`self.SkillTime`))
  (if (`self.IsSkillCoolDown`)
    (`/Game/Blueprints/BP_Timer.SetTargetTime` (`self.BP_Timer`) (`self.SkillTime`))
    (`/Game/Blueprints/BP_Timer.Update` (`self.BP_Timer`) (`GameplayStatics.GetWorldDeltaSeconds`))
    (bind _istimeout (`/Game/Blueprints/BP_Timer.IsTimeOut` (`self.BP_Timer`)))
    (if _istimeout
      (`/Game/Blueprints/BP_Timer.ReSet` (`self.BP_Timer`))
      (set `self.IsSkillCoolDown` false)
      (`Widget.SetVisibility` (`/Game/UI/UMG_Main.SkillCoolDown` (`self.MainUI`)) "HitTestInvisible")
      (else
        (bind _elapsedtime (`/Game/Blueprints/BP_Timer.GetElapsedTime` (`self.BP_Timer`)))
        (set `self.CoolDownValue` (/ (- _skilltime _elapsedtime) _skilltime))
        ;[1 1 1] 파라미터는 인스턴스에서 건들려고 만든거 .. 코드에서 건들려면 다이나믹 머티리얼 호출
        (bind _returnvalue (`Image.GetDynamicMaterial` (`/Game/UI/UMG_Main.SkillCoolDown` (`self.MainUI`))))
        (`MaterialInstanceDynamic.SetScalarParameterValue` _returnvalue "Percent" (`self.CoolDownValue`))))))

(fn `StartSkillCoolDown`
  (set `self.IsSkillCoolDown` true)
  (bind _returnvalue (`Image.GetDynamicMaterial` (`/Game/UI/UMG_Main.SkillCoolDown` (`self.MainUI`))))
  (`MaterialInstanceDynamic.SetScalarParameterValue` _returnvalue "Percent" 1.0)
  (set `self.CoolDownValue` 1.0))

(fn `UserConstructionScript`)