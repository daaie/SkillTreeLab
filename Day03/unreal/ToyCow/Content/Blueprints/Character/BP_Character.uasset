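; Player character Blueprint with tank-style movement, jumping and a montage-based attack.
; UpDown moves along the forward vector, while LeftRight yaws the actor by ROTSpeed scaled with delta time.
; Attack input works only in the default StateBP, switching it to the attack state, playing the "Attack" montage section and printing the state.
; The AttackEnd event restores the default state, allowing the next attack.
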(event `self.ReceiveBeginPlay`)

(event `InputAction|Jump`
  (params (Key :type "Key Structure"))
  (:`Pressed`
    (`self.Jump`)))

(event `InputAxis|UpDown`
  (params (AxisValue :type "Float (single-precision)"))
  (`self.AddMovementInput` (`self.GetActorForwardVector`) AxisValue))

(event `InputAction|Attack`
  (params (Key :type "Key Structure"))
  ;[1 1 1] 공격전환
  (:`Pressed`
    (if (`|EnumEquality` (`self.StateBP`) "NewEnumerator0")
      (set `self.StateBP` "NewEnumerator1")
      (`self.PlayAnimMontage` null 1.0 "Attack")
      (`KismetSystemLibrary.PrintString` (`|GetEnumeratorNameAsString` (`self.StateBP`))))))

(event `InputAxis|LeftRight`
  (params (AxisValue :type "Float (single-precision)"))
  (`self.K2_AddActorLocalRotation` (`KismetMathLibrary.MakeRotator` 0.0 0.0 (* (`GameplayStatics.GetWorldDeltaSeconds`) AxisValue (`self.ROTSpeed`)))))

(event `AttackEnd`
  (set `self.StateBP` "NewEnumerator0"))

(fn `UserConstructionScript`)