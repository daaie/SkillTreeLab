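; Character controller Blueprint that creates the main HUD at BeginPlay and manages a single skill cooldown with its on-screen indicator.
; CanUseSkill reports availability, and StartSkillCooldown locks the skill, shows the indicator and sets BPTimer to SkillTime.
; Tick advances the timer, feeding the remaining fraction into the indicator's dynamic material Percent parameter.
; On timeout it resets the timer, clears the lock and switches the indicator to HitTestInvisible.
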(event `self.ReceiveBeginPlay`
  (bind _returnvalue (`|CreateWidget` "/Game/UI/UMG_Main.UMG_Main_C"))
  (bind _output_get (set `self.MainUI` _returnvalue))
  (`UserWidget.AddToViewport` _output_get 0))

(event `self.ReceiveTick`
  (params (DeltaSeconds :type "Float (single-precision)"))
  (`self.SkillCooldown`))

(fn `CanUseSkill`
  (returns (`Can Skill` :type Boolean))
  (return (not (`self.IsSkillCooldown`))))

(fn `SkillCooldown`
  (bind _skill_time (`self.Skill Time`))
  (if (`self.IsSkillCooldown`)
    (`/Game/Blueprint/Character/BP_Timer.Update` (`self.BP_Timer`) (`GameplayStatics.GetWorldDeltaSeconds`))
    (bind _is_time_out (`/Game/Blueprint/Character/BP_Timer.IsTimeOut` (`self.BP_Timer`)))
    (if _is_time_out
      (`/Game/Blueprint/Character/BP_Timer.Reset` (`self.BP_Timer`))
      (set `self.IsSkillCooldown` false)
      (`Widget.SetVisibility` (`/Game/UI/UMG_Main.SkillCooldown` (`self.MainUI`)) "HitTestInvisible")
      (else
        (bind _elapsed_time (`/Game/Blueprint/Character/BP_Timer.GetElapsedTime` (`self.BP_Timer`)))
        (set `self.CooldownValue` (/ (- _skill_time _elapsed_time) _skill_time))
        (bind _returnvalue (`Image.GetDynamicMaterial` (`/Game/UI/UMG_Main.SkillCooldown` (`self.MainUI`))))
        (`MaterialInstanceDynamic.SetScalarParameterValue` _returnvalue "Percent" (`self.CooldownValue`))))))

(fn `StartSkillCooldown`
  (set `self.IsSkillCooldown` true)
  (`Widget.SetVisibility` (`/Game/UI/UMG_Main.SkillCooldown` (`self.MainUI`)) "Visible")
  (bind _returnvalue (`Image.GetDynamicMaterial` (`/Game/UI/UMG_Main.SkillCooldown` (`self.MainUI`))))
  (`MaterialInstanceDynamic.SetScalarParameterValue` _returnvalue "Percent" 1.0)
  (set `self.CooldownValue` 1.0)
  (`/Game/Blueprint/Character/BP_Timer.SetTargetTime` (`self.BP_Timer`) (`self.Skill Time`)))

(fn `UserConstructionScript`)