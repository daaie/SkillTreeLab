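; BP_Character is a player-controlled character with movement, turning, jumping and a montage-based attack.
; Axis input moves it along its forward vector and yaws it at a frame-time-scaled RotSpeed, giving tank-style controls.
; A StateBP enum gates the attack: the Attack input plays the Warrior montage's Attack section only from the default state, and the AttackEnd event restores that state.
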(event `InputAxis|UpDown`
  (params (AxisValue :type "Float (single-precision)"))
  ;[1 1 1] 이동
  (`self.AddMovementInput` (`self.GetActorForwardVector`) AxisValue))

(event `InputAxis|LeftRight`
  (params (AxisValue :type "Float (single-precision)"))
  ;[1 1 1] 회전
  (`self.K2_AddActorLocalRotation` (`KismetMathLibrary.MakeRotator` 0.0 0.0 (* AxisValue (`GameplayStatics.GetWorldDeltaSeconds`) (`self.RotSpeed`)))))

(event `InputAction|Jump`
  (params (Key :type "Key Structure"))
  ;[1 1 1] 점프
  (:`Pressed`
    (`self.Jump`)))

(event `InputAction|Attack`
  (params (Key :type "Key Structure"))
  ;[1 1 1] 공격 전환
  (:`Pressed`
    (if (`|EnumEquality` (`self.StateBP`) "NewEnumerator0")
      (set `self.StateBP` "NewEnumerator1")
      (`self.PlayAnimMontage` "/Game/Blueprint/Character/Warrior_Montage.Warrior_Montage" 1.0 "Attack"))))

(event `AttackEnd`
  ;[1 1 1] 공격 종료
  (set `self.StateBP` "NewEnumerator0"))

(fn `UserConstructionScript`)