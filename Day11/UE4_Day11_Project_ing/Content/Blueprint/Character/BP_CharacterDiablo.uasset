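; Player character for a Diablo-style action game, with directional movement, melee combo, cooldown-gated skill and HP.
; Tick turns input axes into control rotation and moves along the controller's forward vector unless dead.
; Attack presses play the montage or store the next combo section, while the skill checks its cooldown on BP_CharacterController.
; Separate events handle dash impulse, sphere-trace hits and radial skill damage; AnyDamage reduces HP and sets the death state.
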(event `self.ReceiveBeginPlay`
  ;[1 1 1] 컨트롤러 값 저장.
  (bind _asbp_character_controller (cast `/Game/Blueprint/Character/BP_CharacterController` (`GameplayStatics.GetPlayerController` 0)))
  (set `self.RefController` _asbp_character_controller)
  (set `self.CurrentHP` (`self.MaxHP`)))

(event `self.ReceiveTick`
  (params (DeltaSeconds :type "Float (single-precision)"))
  ;[1 1 1] 캐릭터 이동
  (if (`|EnumInequality` (`self.StateBP`) "NewEnumerator2")
    (if (or (!= (`self.GetInputAxisValue`) 0.0) (!= (`self.GetInputAxisValue`) 0.0))
      (`Controller.SetControlRotation` (`GameplayStatics.GetPlayerController` 0) (`KismetMathLibrary.MakeRotFromX` (`KismetMathLibrary.MakeVector` (`self.GetInputAxisValue`) (`self.GetInputAxisValue`))))
      (`self.AddMovementInput` (`self.GetActorForwardVector` (`GameplayStatics.GetPlayerController` 0))))))

(event `InputAction|Attack`
  (params (Key :type "Key Structure"))
  ;[1 1 1] 공격 전환
  (:`Pressed`
    (set `self.StateBP` "NewEnumerator1" :!label _label)
    (if (`AnimInstance.Montage_IsPlaying` (`SkeletalMeshComponent.GetAnimInstance` (`self.Mesh`)) "/Game/Blueprint/Character/Warrior_Montage.Warrior_Montage")
      (switch `name` (`AnimInstance.Montage_GetCurrentSection` (`SkeletalMeshComponent.GetAnimInstance` (`self.Mesh`)) "/Game/Blueprint/Character/Warrior_Montage.Warrior_Montage")
        (:`Default`
          (set `self.NextSection` "None"))
        (:`Attack1`
          (set `self.NextSection` "Attack2"))
        (:`Attack2`
          (set `self.NextSection` "Attack3"))
        (:`Attack3`
          (set `self.NextSection` "Attack4")))
      (else
        (`AnimInstance.Montage_Play` (`SkeletalMeshComponent.GetAnimInstance` (`self.Mesh`)) "/Game/Blueprint/Character/Warrior_Montage.Warrior_Montage" 1.0 "MontageLength" 0.0 true)))))

(event `DoAttack`
  ;[1 1 1] 공격 전환
  (goto _label))

(event `AttackEnd`
  ;[1 1 1] 공격 종료
  (set `self.StateBP` "NewEnumerator0"))

(event `DoSkill`
  ;[1 1 1] 스킬 공격
  (bind _can_skill (`/Game/Blueprint/Character/BP_CharacterController.CanUseSkill` (`self.RefController`)))
  (if (and (`|EnumEquality` (`self.StateBP`) "NewEnumerator0") _can_skill)
    (set `self.StateBP` "NewEnumerator1")
    (`self.PlayAnimMontage` "/Game/Blueprint/Character/Warrior_Montage.Warrior_Montage" 1.0 "Skill")
    (`/Game/Blueprint/Character/BP_CharacterController.StartSkillCooldown` (`self.RefController`))))

(event `SkillEnd`
  ;[1 1 1] 스킬 종료
  (set `self.StateBP` "NewEnumerator0"))

(event `AttackDash`
  ;[1 1 1] 대쉬 무브
  (`CharacterMovementComponent.AddImpulse` (`self.CharacterMovement`) (* (`self.GetActorForwardVector`) (`self.DashForce`)) true))

(event `AttackHit`
  (bind _returnvalue (`self.K2_GetActorLocation`))
  ;[1 1 1] 공격 판정 및 데이터 전달
  (bind (_outhit _returnvalue_2) (`KismetSystemLibrary.SphereTraceSingleForObjects` :`Start` _returnvalue :`End` (+ _returnvalue (* (`self.GetActorForwardVector`) (`self.AttackRange`))) :`Radius` (`self.AttackRadius`) :`ObjectTypes` (`|MakeArray` "ObjectTypeQuery8" :!type "EObjectTypeQuery Enum") :`DrawDebugType` "ForDuration"))
  (if _returnvalue_2
    (`GameplayStatics.ApplyDamage` (`.HitActor` (`GameplayStatics.BreakHitResult` _outhit)) (`self.AttackDamage`))))

(event `SkillHit`
  ;[1 1 1] 스킬공격판정
  (`GameplayStatics.ApplyRadialDamage` (`self.SkillDamage`) (`self.K2_GetActorLocation`) (`self.SkillRadius`) null (`|MakeArray` self :!type "Actor Object Reference") self (`GameplayStatics.GetPlayerController` 0)))

(event `self.ReceiveAnyDamage`
  (params (Damage :type "Float (single-precision)") (DamageType :type "DamageType Object Reference") (InstigatedBy :type "Controller Object Reference") (DamageCauser :type "Actor Object Reference"))
  (bind _output_get (set `self.CurrentHP` (- (`self.CurrentHP`) Damage)))
  (if (> _output_get 0.0)
    (`KismetSystemLibrary.PrintString` (`KismetStringLibrary.Conv_DoubleToString` (`self.CurrentHP`)))
    (else
      (set `self.StateBP` "NewEnumerator2"))))

(fn `UserConstructionScript`)