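; Enemy AI controller that starts an enemy's behavior tree when it possesses a pawn.
; On possess it loads the enemy blackboard and seeds it with a wait time, the pawn's spawn location as home, and a random navigable point near it as the first target.
; It then runs BP_EnemyBT, which takes over the enemy's decisions.
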(event `self.OnPossess`
  (params (PossessedPawn :type "Pawn Object Reference"))
  (bind _returnvalue (`self.K2_GetActorLocation` (`self.K2_GetPawn`)))
  (`|ExecutionSequence`
    (:`then_0`
      (`self.UseBlackboard` "/Game/Blueprint/Monster/AI/BP_EnemyBB.BP_EnemyBB")
      (`BlackboardComponent.SetValueAsFloat` (`self.Blackboard`) (`self.WaitTimeKey`) 2.0)
      (`BlackboardComponent.SetValueAsVector` (`self.Blackboard`) (`self.HomeLoc`) _returnvalue)
      (`BlackboardComponent.SetValueAsVector` (`self.Blackboard`) (`self.TargetLoc`) (`NavigationSystem.K2_GetRandomLocationInNavigableRadius` _returnvalue 600.0)))
    (:`then_1`
      (`self.RunBehaviorTree` "/Game/Blueprint/Monster/AI/BP_EnemyBT.BP_EnemyBT"))))

(fn `UserConstructionScript`)