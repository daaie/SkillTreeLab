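; BP_EnemyBear is a bear enemy that chases and attacks the Diablo player character.
; A Peace/Chase/Attack/Dead state machine sets walk speed and mirrors state to the Blackboard, alongside the target.
; PawnSensing starts chases, stores the player in Instigator and its sight radius bounds pursuit.
; A sphere toggled by detection start/end events deals damage on overlap; incoming damage updates the HP bar widget and triggers timed death.
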(event `self.ReceiveBeginPlay`
  ;[1 1 1] 초기화
  (set `self.CurrentHP` (`self.MaxHP`))
  (`self.SetState` "NewEnumerator0")
  (`PrimitiveComponent.SetCollisionEnabled` (`self.Sphere`) "NoCollision"))

(event `self.ReceiveTick`
  (params (DeltaSeconds :type "Float (single-precision)"))
  ;[1 1 1] 코멘트
  (switch `/Game/Blueprint/Monster/EBearStates` (`self.StateBP`)
    (:`NewEnumerator0`
      (`self.OnPeace`))
    (:`NewEnumerator1`
      (`self.OnChase`))
    (:`NewEnumerator2`
      (`self.OnAttack`))))

(event `SetState`
  (params (NewState :type "/Game/Blueprint/Monster/EBearStates Enum" :default "NewEnumerator0"))
  (bind _charactermovement (`self.CharacterMovement`))
  ;[1 1 1] 상태 변경 이벤트
  (if (`|EnumInequality` (`self.StateBP`) "NewEnumerator3")
    ;;[1 1 1] 상태 변경 이벤트
    (bind _output_get (set `self.StateBP` NewState))
    (`BlackboardComponent.SetValueAsEnum` (`AIBlueprintHelperLibrary.GetBlackboard` (`self.GetController`)) (`self.StateKey`) _output_get)
    (switch `/Game/Blueprint/Monster/EBearStates` _output_get
      (:`NewEnumerator0`
        (set `CharacterMovementComponent.MaxWalkSpeed` 200.0 _charactermovement))
      (:`NewEnumerator1`
        (set `CharacterMovementComponent.MaxWalkSpeed` 500.0 _charactermovement))
      (:`NewEnumerator2`
        (set `CharacterMovementComponent.MaxWalkSpeed` 0.0 _charactermovement :!label _label))
      (:`NewEnumerator3`
        (goto _label)))))

(event `self.ReceiveAnyDamage`
  (params (Damage :type "Float (single-precision)") (DamageType :type "DamageType Object Reference") (InstigatedBy :type "Controller Object Reference") (DamageCauser :type "Actor Object Reference"))
  ;[1 1 1] 대미지 이벤트
  (set `self.CurrentHP` (- (`self.CurrentHP`) Damage))
  (`self.UpdateHPUI` (`KismetMathLibrary.FTrunc` Damage))
  (if (> (`self.CurrentHP`) 0.0)
    (`KismetSystemLibrary.PrintString` (`KismetStringLibrary.Conv_DoubleToString` (`self.CurrentHP`)))
    (else
      (`self.SetState` "NewEnumerator3")
      (`self.OnDead`))))

(event `UpdateHPUI`
  (params (Damge :type Integer))
  ;[1 1 1] HPBar
  (bind _asumg_hpbar (cast `/Game/UI/UMG_HPBar` (`WidgetComponent.GetUserWidgetObject` (`self.HPBar`))))
  (`/Game/UI/UMG_HPBar.PlayTextAnim` _asumg_hpbar Damge)
  (`/Game/UI/UMG_HPBar.SetHP` _asumg_hpbar (/ (`self.CurrentHP`) (`self.MaxHP`))))

(event `OnPeace`
  ;[1 1 1] 상태 이벤트
)

(event `OnChase`
  ;[1 1 1] 상태 이벤트
  (`self.DistanceCheck`))

(event `self.PawnSensing.OnSeePawn`
  (params (Pawn :type "Pawn Object Reference"))
  ;[1 1 1] 정면 탐지
  (if (`|EnumInequality` (`self.StateBP`) "NewEnumerator3")
    (bind _asbp_character_diablo (cast `/Game/Blueprint/Character/BP_CharacterDiablo` Pawn))
    (if (`|EnumInequality` (`/Game/Blueprint/Character/BP_CharacterDiablo.StateBP` _asbp_character_diablo) "NewEnumerator2")
      ;;[1 1 1] 변수를만들어도되는데 언리얼이 만들어주는 변수도있따
      (bind _output_get (set `self.Instigator` _asbp_character_diablo))
      (`BlackboardComponent.SetValueAsObject` (`AIBlueprintHelperLibrary.GetBlackboard` (`self.GetController`)) (`self.TargetPlayer`) _output_get)
      (`self.SetState` "NewEnumerator1"))))

(event `OnAttack`
  (bind _instigator (`self.Instigator`))
  ;[1 1 1] 상태 이벤트
  (`/Engine/EditorBlueprintResources/StandardMacros.IsValid` _instigator
    (:`Is Valid`
      (bind _asbp_character_diablo (cast `/Game/Blueprint/Character/BP_CharacterDiablo` _instigator))
      (if (`|EnumEquality` (`/Game/Blueprint/Character/BP_CharacterDiablo.StateBP` _asbp_character_diablo) "NewEnumerator2")
        (`self.SetState` "NewEnumerator0")))))

(event `DistanceCheck`
  (bind _instigator (`self.Instigator`))
  ;[1 1 1] 플레이어와 거리체크
  (`/Engine/EditorBlueprintResources/StandardMacros.IsValid` _instigator
    (:`Is Valid`
      (if (> (`KismetMathLibrary.VSize` (- (`self.K2_GetActorLocation` _instigator) (`self.K2_GetActorLocation`))) (`PawnSensingComponent.SightRadius` (`self.PawnSensing`)))
        (`self.SetState` "NewEnumerator0")
        (set `self.Instigator` null)))))

(event `OnDead`
  ;[1 1 1] 상태 이벤트
  (`self.SetLifeSpan` self 2.0)
  (`PrimitiveComponent.SetCollisionEnabled` (`self.CapsuleComponent`) "NoCollision")
  (bind _asumg_hpbar (cast `/Game/UI/UMG_HPBar` (`WidgetComponent.GetUserWidgetObject` (`self.HPBar`))))
  (`/Game/UI/UMG_HPBar.SetHP` _asumg_hpbar 0.0))

(event `AttackDetectStart`
  ;[1 1 1] 공격 감지 시작
  (`PrimitiveComponent.SetCollisionEnabled` (`self.Sphere`) "QueryOnly"))

(event `AttackDetectEnd`
  ;[1 1 1] 공격 감지 종료
  (`PrimitiveComponent.SetCollisionEnabled` (`self.Sphere`) "NoCollision"))

(event `self.Sphere.OnComponentBeginOverlap`
  (params (OverlappedComponent :type "PrimitiveComponent Object Reference") (OtherActor :type "Actor Object Reference") (OtherComp :type "PrimitiveComponent Object Reference") (OtherBodyIndex :type Integer) (bFromSweep :type Boolean) (SweepResult :type "HitResult Structure (by ref)"))
  (`GameplayStatics.ApplyDamage` OtherActor (`self.Attack`) (`self.GetController`) self))

(fn `UserConstructionScript`)