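; BP_Female is a character Blueprint that handles player input for movement, sprinting, jumping, camera zoom and attacking.
; Movement follows control-rotation yaw and is blocked while IsAttack is set; Fire sets that flag, and nothing here clears it.
; Sprint swaps max walk speed with the value cached at BeginPlay, and Zoom changes spring arm length.
; Turn and LookUp are empty, with their controller-input nodes disconnected.
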(event `self.ReceiveBeginPlay`
  (set `self.WalkSpeed` (`CharacterMovementComponent.MaxWalkSpeed` (`self.CharacterMovement`))))

(event `InputAction|Sprint`
  (params (Key :type "Key Structure"))
  (:`Pressed`
    (set `CharacterMovementComponent.MaxWalkSpeed` (`self.RunSpeed`) (`self.CharacterMovement`)))
  (:`Released`
    (set `CharacterMovementComponent.MaxWalkSpeed` (`self.WalkSpeed`) (`self.CharacterMovement`))))

(event `InputAxis|MoveForward`
  (params (AxisValue :type "Float (single-precision)"))
  (bind (_returnvalue_roll _returnvalue_pitch _returnvalue_yaw) (`KismetMathLibrary.BreakRotator` (`self.GetControlRotation`)))
  (if (not (`self.IsAttack`))
    (`self.AddMovementInput` (`KismetMathLibrary.GetForwardVector` (`KismetMathLibrary.MakeRotator` 0.0 0.0 _returnvalue_yaw)) AxisValue)))

(event `InputAxis|Turn`
  (params (AxisValue :type "Float (single-precision)")))

(event `InputAxis|MoveRight`
  (params (AxisValue :type "Float (single-precision)"))
  (bind (_returnvalue_roll _returnvalue_pitch _returnvalue_yaw) (`KismetMathLibrary.BreakRotator` (`self.GetControlRotation`)))
  (if (not (`self.IsAttack`))
    (`self.AddMovementInput` (`KismetMathLibrary.GetRightVector` (`KismetMathLibrary.MakeRotator` 0.0 0.0 _returnvalue_yaw)) AxisValue)))

(event `InputAxis|LookUp`
  (params (AxisValue :type "Float (single-precision)")))

(event `InputAxis|Zoom`
  (params (AxisValue :type "Float (single-precision)"))
  (set `SpringArmComponent.TargetArmLength` (+ AxisValue (`SpringArmComponent.TargetArmLength` (`self.SpringArm`))) (`self.SpringArm`)))

(event `InputAction|Jump`
  (params (Key :type "Key Structure"))
  (:`Pressed`
    (`self.Jump`)
    (set `self.IsJumping` true))
  (:`Released`
    (`self.StopJumping`)
    (set `self.IsJumping` false)))

(event `InputAction|Fire`
  (params (Key :type "Key Structure"))
  (:`Pressed`
    (set `self.IsAttack` true)))

(fn `UserConstructionScript`)